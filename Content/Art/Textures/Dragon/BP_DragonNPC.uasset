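; Dragon NPC that wakes from sleep and starts a linear dialogue when the player first enters its collision.
; After a short delay it stops looping the current flipbook, then chains flipbook changes through finished-playing events: sleep-to-stand, then a looping stand-to-idle.
; A timeline lerps the flipbook's position by an offset during the rise, and dialogue begins shortly after the idle flipbook starts.
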(event OnComponentBeginOverlap(Collision)
  (params (OverlappedComponent :type Primitive%20Component%20Object%20Reference) (OtherActor :type Actor%20Object%20Reference) (OtherComp :type Primitive%20Component%20Object%20Reference) (OtherBodyIndex :type Integer) (bFromSweep :type Boolean) (SweepResult :type Hit%20Result%20Structure%20%28by%20ref%29))
  (bind _paperflipbook (Variables|Default|GetPaperFlipbook))
  (Utilities|Casting|CastToBP_PlayerCharacter OtherActor)
  (Utilities|FlowControl|DoOnce false
    (:Completed
      (Utilities|FlowControl|Delay 1.0)
      (EventDispatchers|BindEventtoOnFinishedPlaying _paperflipbook (delegate Custom|SleepToStand))
      (Components|Timeline|SetLooping _paperflipbook false))))

(event Custom|SleepToStand
  (bind _paperflipbook (Variables|Default|GetPaperFlipbook))
  (bind _startloc (Variables|Default|GetStartLoc))
  (Utilities|FlowControl|Sequence
    (:then_0
      (bind _alpha (Timeline|OffsetFlipbook Play)
        (:Update
          (Transformation|SetRelativeLocation (Variables|Default|GetPaperFlipbook) (Math|Vector|Lerp(Vector) _startloc (+ _startloc (Variables|Default|GetOffset)) _alpha) false false))))
    (:then_1
      (Sprite|SetFlipbook _paperflipbook "/Game/Art/Textures/Dragon/DragonSleepToStand/SleepToStand.SleepToStand")
      (Audio|Components|Audio|Play _paperflipbook)
      (EventDispatchers|BindEventtoOnFinishedPlaying (Variables|Default|GetPaperFlipbook) (delegate Custom|StandToIdle)))))

(event Custom|StandToIdle
  (bind _paperflipbook (Variables|Default|GetPaperFlipbook))
  (Sprite|SetFlipbook _paperflipbook "/Game/Art/Textures/Dragon/DragonStandToIdle/StandToIdle.StandToIdle")
  (Audio|Components|Audio|Play _paperflipbook)
  (Components|Timeline|SetLooping (Variables|Default|GetPaperFlipbook) true)
  (Utilities|FlowControl|Delay 2.0)
  (Default|StartDialogue (Variables|Default|GetAC_Dialogue_Linear_Dragon)))

(event EventBeginPlay
  (Variables|Default|SetStartLoc (Variables|/Script/Engine.SceneComponent|GetRelativeLocation (Variables|Default|GetPaperFlipbook))))

(fn ConstructionScript)