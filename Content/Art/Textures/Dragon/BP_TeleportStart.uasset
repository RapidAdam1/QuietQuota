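; BP_TeleportStart is a trigger actor that moves the player character to a referenced TeleportLocation actor when the character overlaps its Box.
; On overlap it fades the camera out, toggles the player's animation update flag, clears movement input and disables input.
; After short delays hide the location change, it fades back in and restores animation and input.
; The player reference is cached at BeginPlay, with the overlap cast serving only as a filter.
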(event OnComponentBeginOverlap(Box)
  (params (OverlappedComponent :type Primitive%20Component%20Object%20Reference) (OtherActor :type Actor%20Object%20Reference) (OtherComp :type Primitive%20Component%20Object%20Reference) (OtherBodyIndex :type Integer) (bFromSweep :type Boolean) (SweepResult :type Hit%20Result%20Structure%20%28by%20ref%29))
  (bind _asbp_player_character (Utilities|Casting|CastToBP_PlayerCharacter OtherActor))
  (CameraFades|StartCameraFade :self (Variables|/Script/Engine.PlayerController|GetPlayerCameraManager (Game|GetPlayerController 0)) :ToAlpha 1.0 :Duration 0.5 :bHoldWhenFinished true)
  (Default|UpdateAnimation (Variables|Default|GetPlayer) true)
  (Variables|/Game/Core/PlayerCharacter/BP_PlayerCharacter.BP_PlayerCharacter_C|SetInputValues (Variables|Default|GetPlayer) "")
  (Input|DisableInput (Variables|Default|GetPlayer) (Game|GetPlayerController 0))
  (Utilities|FlowControl|Delay 0.5)
  (Transformation|SetActorLocation (Variables|Default|GetPlayer) (Transformation|GetActorLocation (Variables|Default|GetTeleportLocation)) false false)
  (Utilities|FlowControl|Delay 0.5)
  (CameraFades|StartCameraFade :self (Variables|/Script/Engine.PlayerController|GetPlayerCameraManager (Game|GetPlayerController 0)) :FromAlpha 1.0 :ToAlpha 0.0 :Duration 0.5 :bHoldWhenFinished true)
  (Default|UpdateAnimation (Variables|Default|GetPlayer) false)
  (Input|EnableInput (Variables|Default|GetPlayer) (Game|GetPlayerController 0)))

(event EventBeginPlay
  (bind _returnvalue (Actor|GetActorOfClass "/Game/Core/PlayerCharacter/BP_PlayerCharacter.BP_PlayerCharacter_C"))
  (Variables|Default|SetPlayer _returnvalue))

(fn ConstructionScript)