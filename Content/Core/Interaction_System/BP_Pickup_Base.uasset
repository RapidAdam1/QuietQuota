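; BP_Pickup_Base is a base pickup Blueprint that can be flagged as an objective target and marked on the minimap.
; SetasObjectiveTarget adds an AC_Minimap_Collect component at runtime when the flag is true, storing it as MinimapIcon, and destroys that component when false.
; The construction script is empty, and the CallOnPickup call sits in the event graph without ever running.
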(event EventSetasObjectiveTarget
  (params (SetAsTarget :type Boolean))
  (if SetAsTarget
    (CallFunction|AddMinimapIcon)
    (else
      (CallFunction|RemoveMinimapIcon))))

(fn ConstructionScript)

(fn AddMinimapIcon
  (bind _returnvalue (Game|AddComponentbyClass "/Game/Core/Minimap/AC_Minimap_Collect.AC_Minimap_Collect_C" false))
  (Variables|Default|SetMinimapIcon _returnvalue))

(fn RemoveMinimapIcon
  (Utilities|IsValid (Variables|Default|GetMinimapIcon)
    (:Is%20Valid
      (Components|DestroyComponent (Variables|Default|GetMinimapIcon)))))