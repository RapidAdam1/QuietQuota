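; BP_Level_Informant is a level informant actor that starts the objectives when the player walks into its box.
; The first overlap passes a DoOnce before the player cast, then removes the minimap icon and calls StartObjectives on the BP_ObjectiveManager found in the world.
; It overrides AddMinimapIcon to attach a scaled informant minimap component, and leaves OnInteract_2 empty to suppress the parent's interaction.
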(event OnComponentBeginOverlap(Box)
  (params (OverlappedComponent :type Primitive%20Component%20Object%20Reference) (OtherActor :type Actor%20Object%20Reference) (OtherComp :type Primitive%20Component%20Object%20Reference) (OtherBodyIndex :type Integer) (bFromSweep :type Boolean) (SweepResult :type Hit%20Result%20Structure%20%28by%20ref%29))
  (Utilities|FlowControl|DoOnce false
    (:Completed
      (Utilities|Casting|CastToBP_PlayerCharacter OtherActor)
      (CallFunction|RemoveMinimapIcon)
      (bind _returnvalue (Actor|GetActorOfClass "/Game/Core/AdvancedObjectives/BP_ObjectiveManager.BP_ObjectiveManager_C"))
      (Default|StartObjectives _returnvalue))))

(event Custom|OnInteract_2
  (params (InteractingPlayer :type BP%20Player%20Character%20Object%20Reference))
  ;[1 1 1] Leave in to override parent
)

(fn ConstructionScript
  (|CallParentFunction))

(fn AddMinimapIcon
  (bind _returnvalue (Game|AddComponentbyClass "/Game/Core/Minimap/AC_Minimap_Informant.AC_Minimap_Informant_C" false (Math|Transform|MakeTransform "0, 0, 0" "0, 0, 0" (Math|Vector|MakeVector 4.0 4.0 1.0))))
  (Variables|Default|SetMinimapIcon _returnvalue))