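; BP_SafeRoomInformant is an interactable safe room informant whose dialogue unlocks the player's ability to leave.
; Until first used, interactability changes toggle its prompt widget and end any linear safe room dialogue.
; Interacting sets the player's CanLeave flag, hides the prompt, marks the informant as used, starts the dialogue and broadcasts OnInformantSpokenTo.
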(event EventCanInteract
  (params (CanInteract :type Boolean))
  (if (not (Variables|Default|GetHasInteracted))
    (Development|SetHiddeninGame (Variables|Default|GetInteractWidget) (not CanInteract) false)
    (Default|EndDialogue (Variables|Default|GetAC_Dialogue_Linear_SafeRoom))))

(event EventOnInteract
  (params (PlayerRef :type BP%20Player%20Character%20Object%20Reference))
  (bind _output_get (Variables|Default|SetPlayer PlayerRef))
  (Variables|/Game/Core/PlayerCharacter/BP_PlayerCharacter.BP_PlayerCharacter_C|SetCanLeave _output_get true)
  (Development|SetHiddeninGame (Variables|Default|GetInteractWidget) true true)
  (Variables|Default|SetHasInteracted true)
  (Default|StartDialogue (Variables|Default|GetAC_Dialogue_Linear_SafeRoom))
  (Default|CallOnInformantSpokento))

(fn ConstructionScript
  (|CallParentFunction))