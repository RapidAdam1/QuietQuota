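; Player detection component that tracks an awareness level from the AI controllers currently perceiving the owning character.
; A looping timer raises awareness by a summed, distance-mapped rate per perceiver, or decays it when the character is unseen or undetectable.
; Crouching halves gain and doubles decay.
; Each update broadcasts awareness changes, and reaching maximum while seen alerts all perceivers and fires a player-detected event.
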(event Custom|Init
  (params (OwningCharacter :type BP%20Player%20Character%20Object%20Reference))
  (Variables|Default|SetOwning%20Character OwningCharacter)
  (Utilities|Time|SetTimerbyEvent (delegate Custom|Assess%20Detection) (Variables|Default|GetDetection%20Interval) true))

(event Custom|AlertAllEnemiesInSight
  (for _array_element (Variables|Default|GetPercievedBy)
    (Default|OnAlerted _array_element true)))

(event Custom|RemovePercieving
  (params (PercieverController :type Enemy%20Controller%20Base%20Object%20Reference))
  (Utilities|Array|RemoveItem (Variables|Default|GetPercievedBy) PercieverController))

(event Custom|AddPerceiving
  (params (PercieverController :type Enemy%20Controller%20Base%20Object%20Reference))
  (Utilities|Array|AddUnique (Variables|Default|GetPercievedBy) PercieverController))

(event Custom|Assess%20Detection
  (if (Variables|Default|GetCanBeDetected)
    (if (!= (Utilities|Array|Length (Variables|Default|GetPercievedBy)) 0)
      ;[1 1 1] Seen
      (Variables|Default|SetCurrentAwareness (Math|Float|Clamp(Float) (+ (Variables|Default|GetCurrentAwareness) (CallFunction|CalculateDetectionRate)) 0.0 (Variables|Default|GetMaxAwareness)))
      (Utilities|FlowControl|Sequence
        (:then_0
          (if (== (Variables|Default|GetCurrentAwareness) (Variables|Default|GetMaxAwareness))
            (CallFunction|AlertAllEnemiesinSight)
            (Default|CallOnPlayerDetected)))
        (:then_1
          (Default|CallOnAwarenessChanged (Variables|Default|GetCurrentAwareness) (Variables|Default|GetMaxAwareness) :!label _label)))
      (else
        ;[1 1 1] Unseen
        (if (Variables|/Script/Engine.Character|GetbIsCrouched (Variables|Default|GetOwning%20Character)) :!label _label_2
          (Variables|Default|SetCurrentAwareness (Math|Float|Clamp(Float) (- (Variables|Default|GetCurrentAwareness) (* (Variables|Default|GetDetectionLossRate) 2.0)) 0.0 (Variables|Default|GetMaxAwareness)))
          (goto _label)
          (else
            (Variables|Default|SetCurrentAwareness (Math|Float|Clamp(Float) (- (Variables|Default|GetCurrentAwareness) (Variables|Default|GetDetectionLossRate)) 0.0 (Variables|Default|GetMaxAwareness)))
            (goto _label)))))
    (else
      (goto _label_2))))

(fn CalculateDetectionRate
  ;[1 1 1] Calculate Detection on Seen
  (LocalVariables|SetCurrDetectionRate 0.0)
  (if (!= (Utilities|Array|Length (Variables|Default|GetPercievedBy)) 0)
    (for _array_element (Variables|Default|GetPercievedBy)
      (LocalVariables|SetCurrDetectionRate (+ (LocalVariables|GetCurrDetectionRate) (Math|Float|MapRangeClamped (Transformation|GetDistanceTo (Variables|Default|GetOwning%20Character) _array_element) 0.0 (Variables|/Game/Core/AI/Enemy_ControllerBase.Enemy_ControllerBase_C|GetDetectionDistance _array_element) 1.0 0.0))))
    (if (Variables|/Script/Engine.Character|GetbIsCrouched (Variables|Default|GetOwning%20Character))
      (LocalVariables|SetCurrDetectionRate (/ (LocalVariables|GetCurrDetectionRate) 2.0)))
    (return (LocalVariables|GetCurrDetectionRate))
    (else
      (return 0.0))))