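; BP_Chest is an interactable loot chest that gives the player one key and a small random amount of currency.
; Init, when passed HasKey, activates a sparkle effect and caches the lid's starting rotation.
; OnInteract marks it open, plays sounds and an emitter, pays the cached player, and swings the lid via timeline.
; CanInteract toggles the prompt widget, showing it only while the chest is closed.
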(event Custom|Init
  (params (Has%20Key :type Boolean))
  ;[1 1 1] Init Chain
  (if Has%20Key
    (Components|Activation|Activate (Variables|Default|GetNS_Sparkle) false)
    (Variables|Default|SetLidStartingRot (Variables|/Script/Engine.SceneComponent|GetRelativeRotation (Variables|Default|GetPivot)))))

(event EventBeginPlay
  (bind _returnvalue (Actor|GetActorOfClass "/Game/Core/PlayerCharacter/BP_PlayerCharacter.BP_PlayerCharacter_C"))
  (Variables|Default|SetPlayer _returnvalue))

(event EventOnInteract
  (params (PlayerRef :type BP%20Player%20Character%20Object%20Reference))
  (bind _lidstartingrot (Variables|Default|GetLidStartingRot))
  (Variables|Default|SetIsOpen true)
  (Development|SetHiddeninGame (Variables|Default|GetBPW_InteractPrompt) true false)
  (Utilities|FlowControl|Sequence
    (:then_0
      ;[1 1 1] Feedback
      (Audio|PlaySound2D 0 1.0 1.0 0.0 0 0)
      (Effects|SpawnEmitteratLocation 0 (Transformation|GetWorldLocation (Variables|Default|GetNS_EmitterLocationArrow))))
    (:then_1
      (Default|AlterKeys (Variables|Default|GetPlayer) 1)
      (Default|AlterCurrency (Variables|Default|GetPlayer) (Math|Random|RandomIntegerinRange 5 10)))
    (:then_2
      ;[1 1 1] OpenChestLid
      (bind _rotationalpha (Timeline|OpenChestTimeline Play)
        (:Update
          (Transformation|SetRelativeRotation (Variables|Default|GetPivot) (Math|Rotator|Lerp(Rotator) (Variables|Default|GetLidStartingRot) (Math|Rotator|MakeRotator -5e+01 (.pitch _lidstartingrot) (.yaw _lidstartingrot)) _rotationalpha true) false false))))
    (:then_3
      (Audio|PlaySound2D "/Game/UI/UI_Audio/OpenDoorChest_Cue.OpenDoorChest_Cue" 1.0 1.0 0.0 0 0))))

(event EventCanInteract
  (params (CanInteract :type Boolean))
  ;[1 1 1] Can Interact Check
  (if CanInteract
    (if (not (Variables|Default|GetIsOpen))
      (Development|SetHiddeninGame (Variables|Default|GetBPW_InteractPrompt) (not CanInteract) false :!label _label))
    (else
      (goto _label))))

(fn ConstructionScript)