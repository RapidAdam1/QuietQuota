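; AC_Health is a health component that tracks a current health value and applies damage to it.
; On BeginPlay it stores the current value as the starting value.
; TakeDamage subtracts damage with a floor of zero and calls OnDead whenever the result is zero.
; It then returns the remaining health along with a normalized value relative to the starting health.
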(event EventBeginPlay
  (Variables|Default|SetStartValue (Variables|Default|GetCurrentValue)))

(fn TakeDamage
  (params (DamageValue :type Float%20%28double-precision%29))
  (Variables|Default|SetCurrentValue (Math|Float|Clamp(Float) (- (Variables|Default|GetCurrentValue) DamageValue) 0.0 1e+06))
  (Utilities|FlowControl|Sequence
    (:then_0
      (if (<= (Variables|Default|GetCurrentValue) 0.0)
        (Default|CallOnDead)))
    (:then_1
      (return (Variables|Default|GetCurrentValue) (Math|Float|MapRangeClamped (Variables|Default|GetCurrentValue) 0.0 (Variables|Default|GetStartValue) 0.0 1.0)))))