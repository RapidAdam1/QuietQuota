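; BP_SafeRoomExit is the safe room exit trigger that offers the player a way to leave the level.
; When a player character with CanLeave set overlaps its Box, it creates and shows the WBP_ExitLevel widget.
; It also caches the game instance and sets InfoRecieved when the Informant is spoken to.
; The branch that checks InfoRecieved before calling LoadLevel is disconnected, so that flag does not gate the exit.
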(event OnComponentBeginOverlap(Box)
  (params (OverlappedComponent :type Primitive%20Component%20Object%20Reference) (OtherActor :type Actor%20Object%20Reference) (OtherComp :type Primitive%20Component%20Object%20Reference) (OtherBodyIndex :type Integer) (bFromSweep :type Boolean) (SweepResult :type Hit%20Result%20Structure%20%28by%20ref%29))
  (bind _asbp_player_character (Utilities|Casting|CastToBP_PlayerCharacter OtherActor))
  (if (Variables|/Game/Core/PlayerCharacter/BP_PlayerCharacter.BP_PlayerCharacter_C|GetCanLeave _asbp_player_character)
    (bind _returnvalue (UserInterface|CreateWidget "/Game/UI/WBP_ExitLevel.WBP_ExitLevel_C"))
    (UserInterface|Viewport|AddtoViewport _returnvalue 0)))

(event Custom|SetLock
  (Variables|Default|SetInfoRecieved true))

(event EventBeginPlay
  (EventDispatchers|BindEventtoOnInformantSpokento (Variables|Default|GetInformant) (delegate Custom|SetLock))
  (bind _asgi_quiet_quota_instance (Utilities|Casting|CastToGI_QuietQuota_Instance (Game|GetGameInstance)))
  (Variables|Default|SetGameInstanceRef _asgi_quiet_quota_instance))

(fn ConstructionScript)