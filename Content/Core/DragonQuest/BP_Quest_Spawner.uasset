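; Quest manager that runs a three-step chain: informant, a randomly chosen assassinate or thief job, then a return to the player's recorded start location.
; Each step reads DT_QuestData, targets a random placed actor or spawns the return item, binds its completion event and broadcasts the assignment.
; Finishing the chain once awards currency, disables input, then after a delay saves and loads a level through the game instance.
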(event Custom|GenerateMainQuest
  ;[1 1 1] Generate Main Quest
  (if (== (Math|Random|RandomBool) true)
    (bind _returnvalue (Utilities|GetDataTableRow "/Game/Core/DragonQuest/DT_QuestData.DT_QuestData" "Assassinate")
      (:then
        (CallFunction|SetRandomQuest _returnvalue)))
    (else
      (bind _returnvalue_2 (Utilities|GetDataTableRow "/Game/Core/DragonQuest/DT_QuestData.DT_QuestData" "Thief")
        (:then
          (CallFunction|SetRandomQuest _returnvalue_2))))))

(event Custom|GenerateReturnQuest
  ;[1 1 1] Generate Return Quest
  (bind _returnvalue (Utilities|GetDataTableRow "/Game/Core/DragonQuest/DT_QuestData.DT_QuestData" "End")
    (:then
      (bind _returnvalue_2 (Game|SpawnActorfromClass (.QuestClass (Utilities|Struct|BreakFQuestData _returnvalue)) (Math|Transform|MakeTransform (Variables|Default|GetPlayerStartLocation) "0, 0, 0" "1.000000,1.000000,1.000000") "AdjustIfPossibleButAlwaysSpawn" "MultiplyWithRoot" 0 0))
      (CallFunction|SeLinearQuest _returnvalue_2 _returnvalue))))

(event Custom|GenerateInformantQuest
  ;[1 1 1] Generate Informant Quest
  (bind _returnvalue (Utilities|GetDataTableRow "/Game/Core/DragonQuest/DT_QuestData.DT_QuestData" "Informant")
    (:then
      (CallFunction|SetRandomQuest _returnvalue))))

(event Custom|SelectQuest
  ;[1 1 1] Select Quest
  (switch int (Variables|Default|GetQuestIndex)
    (:0
      (CallFunction|GenerateInformantQuest))
    (:1
      (CallFunction|GenerateMainQuest))
    (:2
      (CallFunction|GenerateReturnQuest))
    (:3
      (CallFunction|OnQuestsCompleted))))

(event Custom|OnTaskCompleted
  ;[1 1 1] On Task Completed
  (Variables|Default|SetQuestIndex (+ (Variables|Default|GetQuestIndex) 1))
  (CallFunction|SelectQuest))

(event Custom|StartQuests
  ;[1 1 1] Start Quests
  (CallFunction|SelectQuest)
  (Variables|Default|SetPlayerStartLocation (Transformation|GetActorLocation (Game|GetPlayerCharacter 0))))

(event Custom|OnQuestsCompleted
  (bind _returnvalue (Game|GetPlayerCharacter 0))
  ;[1 1 1] On Quest Completed
  (Utilities|FlowControl|DoOnce false
    (:Completed
      (bind _asbp_player_character (Utilities|Casting|CastToBP_PlayerCharacter _returnvalue))
      (Default|AlterCurrency _asbp_player_character 100)
      (Input|DisableInput _returnvalue (Game|GetPlayerController 0))
      (Utilities|FlowControl|Delay 2.0)
      (bind _asgi_quiet_quota_instance (Utilities|Casting|CastToGI_QuietQuota_Instance (Game|GetGameInstance)))
      (Default|SaveData _asgi_quiet_quota_instance true)
      (Default|LoadLevel _asgi_quiet_quota_instance "NewEnumerator0"))))

(fn ConstructionScript)

(fn SetRandomQuest
  (params (QuestDetails :type F%20Quest%20Data%20Structure))
  (bind _outactors (Actor|GetAllActorsOfClass (.QuestClass (Utilities|Struct|BreakFQuestData QuestDetails))))
  (bind _output_get (Variables|Default|SetQuestItems _outactors))
  (bind _asbp_base_quest_item (Utilities|Casting|CastToBP_Base_Quest_Item (Utilities|Array|Get(acopy) (Variables|Default|GetQuestItems) (Class|KismetMathLibrary|RandomIntegerfromStream (Math|Random|MakeRandomStream (Math|Random|RandomIntegerinRange 0 100)) (- (Utilities|Array|Length _output_get) 1)))))
  (Default|SetasQuestTarget _asbp_base_quest_item true)
  (EventDispatchers|BindEventtoOnQuestTaskCompleted _asbp_base_quest_item (EventDispatchers|CreateEvent :!event Custom|OnTaskCompleted))
  (Default|CallOnQuestAssigned QuestDetails)
  (return))

(fn SeLinearQuest
  (params (QuestItem :type BP%20Base%20Quest%20Item%20Object%20Reference) (QuestData :type F%20Quest%20Data%20Structure))
  (Default|SetasQuestTarget QuestItem true)
  (EventDispatchers|BindEventtoOnQuestTaskCompleted QuestItem (EventDispatchers|CreateEvent :!event Custom|OnTaskCompleted))
  (Default|CallOnQuestAssigned QuestData))