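; Base quest pickup actor that shows a sprite and completes a quest task when interacted with, then destroys itself.
; It stays hidden without collision until SetAsQuestTarget activates it, and CanInteract toggles the interact prompt's visibility.
; While it is a target, AddMiniMapIcon spawns an icon component above the sprite and registers it in the SceneCapture2D show-only list.
; Interaction unregisters and destroys that icon before removing the actor.
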(event EventBeginPlay
  (Rendering|Components|Sprite|SetSprite (Variables|Default|GetPaperSprite) (Variables|Default|GetSpriteItem))
  (CallFunction|SetasQuestTarget false))

(event EventOnInteract
  (params (PlayerRef :type BP%20Player%20Character%20Object%20Reference))
  (if (Variables|Default|GetIsQuestItem)
    (Variables|Default|SetIsQuestItem false)
    (Default|CallOnQuestTaskCompleted)
    (CallFunction|RemoveMiniMapIcon)
    (Actor|DestroyActor)))

(event EventCanInteract
  (params (CanInteract :type Boolean))
  (Development|SetHiddeninGame (Variables|Default|GetBPW_InteractPrompt) (not CanInteract) false))

(fn ConstructionScript
  (Rendering|Components|Sprite|SetSprite (Variables|Default|GetPaperSprite) (Variables|Default|GetSpriteItem)))

(fn SetasQuestTarget
  (params (SetTrue :type Boolean))
  (bind _output_get (Variables|Default|SetIsQuestItem SetTrue))
  (if _output_get
    (Collision|SetCollisionEnabled (Variables|Default|GetBox) "QueryAndPhysics")
    (Development|SetHiddeninGame (Variables|Default|GetPaperSprite) false false)
    (else
      (Collision|SetCollisionEnabled (Variables|Default|GetBox) "NoCollision")
      (Development|SetHiddeninGame (Variables|Default|GetPaperSprite) true false))))

(fn AddMiniMapIcon
  (params (MinimapIcon :type AC%20Minimap%20Base%20Class%20Reference))
  (if (Variables|Default|GetIsQuestItem)
    (bind _returnvalue (Game|AddComponentbyClass MinimapIcon true (Math|Transform|MakeTransform "0, 0, 0" "0, 0, 0" "10.000000,10.000000,1.000000")))
    (bind _output_get (Variables|Default|SetMinimapIcon _returnvalue))
    (bind _returnvalue_2 (Actor|GetActorOfClass "/Script/Engine.SceneCapture2D"))
    (Rendering|SceneCapture|ShowOnlyComponent (Variables|/Script/Engine.SceneCapture2D|GetCaptureComponent2D _returnvalue_2) _output_get)
    (Transformation|SetWorldLocation _output_get (+ (Transformation|GetWorldLocation (Variables|Default|GetPaperSprite)) "0.000000,0.000000,410.000000") false false)))

(fn RemoveMiniMapIcon
  (Utilities|IsValid (Variables|Default|GetMinimapIcon)
    (:Is%20Valid
      (bind _returnvalue (Actor|GetActorOfClass "/Script/Engine.SceneCapture2D"))
      (Class|SceneCaptureComponent|RemoveShowOnlyComponent (Variables|/Script/Engine.SceneCapture2D|GetCaptureComponent2D _returnvalue) (Variables|Default|GetMinimapIcon))
      (Components|DestroyComponent (Variables|Default|GetMinimapIcon)))))