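; BP_Thief_Item is an interactable item that can serve as a collectible quest target, extending a parent item class.
; Setting it as a quest target adds a collect minimap icon regardless of the flag, then toggles its Niagara effect to match.
; On interact, after the parent logic, a quest item stops the effect, plays a collect sound and destroys itself.
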(event EventBeginPlay
  (|CallParentFunction))

(event Collision|EventActorBeginOverlap
  (params (OtherActor :type Actor%20Object%20Reference)))

(event EventTick
  (params (DeltaSeconds :type Float%20%28single-precision%29)))

(event EventOnInteract
  (params (PlayerRef :type BP%20Player%20Character%20Object%20Reference))
  (|CallParentFunction PlayerRef)
  (if (Variables|Default|GetIsQuestItem)
    (Components|Activation|Deactivate (Variables|Default|GetNiagara))
    (Audio|PlaySound2D "/Game/UI/UI_Audio/CollectValuable_Cue.CollectValuable_Cue" 1.0 1.0 0.0 0 0)
    (Actor|DestroyActor)))

(fn ConstructionScript
  (|CallParentFunction))

(fn SetasQuestTarget
  (params (SetTrue :type Boolean))
  (|CallParentFunction SetTrue)
  (CallFunction|AddMiniMapIcon "/Game/Core/Minimap/AC_Minimap_Collect.AC_Minimap_Collect_C")
  (if SetTrue
    (Components|Activation|Activate (Variables|Default|GetNiagara) false)
    (else
      (Components|Activation|Deactivate (Variables|Default|GetNiagara)))))