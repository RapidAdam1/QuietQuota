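; BP_Assassinate_Item is an interactable item for assassinate quests, built on a parent item class.
; When it is a quest item, interacting plays a 2D death sound and destroys the actor after the parent logic runs.
; CanInteract shows or hides the interact prompt widget for quest items, and SetAsQuestTarget adds an assassinate minimap icon after calling the parent.
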(event EventBeginPlay
  (|CallParentFunction) ; This node is disabled and will not be called.\nDrag off pins to build functionality.
)

(event Collision|EventActorBeginOverlap
  (params (OtherActor :type Actor%20Object%20Reference)))

(event EventTick
  (params (DeltaSeconds :type Float%20%28single-precision%29)))

(event EventOnInteract
  (params (PlayerRef :type BP%20Player%20Character%20Object%20Reference))
  (|CallParentFunction PlayerRef)
  (if (Variables|Default|GetIsQuestItem)
    (Audio|PlaySound2D "/Game/UI/UI_Audio/Death_Cue.Death_Cue" 1.0 1.0 0.0 0 0)
    (Actor|DestroyActor)))

(event EventCanInteract
  (params (CanInteract :type Boolean))
  (if (Variables|Default|GetIsQuestItem)
    (Development|SetHiddeninGame (Variables|Default|GetBPW_InteractPrompt) (not CanInteract) false)))

(fn ConstructionScript
  (|CallParentFunction))

(fn SetasQuestTarget
  (params (SetTrue :type Boolean))
  (|CallParentFunction SetTrue)
  (CallFunction|AddMiniMapIcon "/Game/Core/Minimap/AC_Minimap_Assassinate.AC_Minimap_Assassinate_C"))