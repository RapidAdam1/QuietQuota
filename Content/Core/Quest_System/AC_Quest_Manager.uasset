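; AC_Quest_Manager is a quest manager that tracks a single active quest.
; On Initialize it binds a completion callback to every BP_Target actor in the level.
; NewQuest overwrites the current quest and clears on-screen debug messages; its clue print has screen and log output disabled.
; GetQuest exposes the current state, and OnNewQuestCompleted clears the quest when the completed ID matches.
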(event Custom|Initialize
  (bind _outactors (Actor|GetAllActorsOfClass "/Game/Core/ObjectiveSystem/Items/BP_Target.BP_Target_C"))
  (for _array_element _outactors
    (EventDispatchers|BindEventtoOnQuestCompleted _array_element (EventDispatchers|CreateEvent :!event OnNewQuestCompleted))))

(fn NewQuest
  (params (quest :type S%20Quest%20Details%20Structure))
  (Variables|Default|SetCurrentQuest quest)
  (Variables|Default|SetHasQuest true)
  (Development|ExecuteConsoleCommand "ClearOnScreenDebugMessages" 0)
  (Development|PrintString (Utilities|Struct|BreakS_QuestDetails (Variables|Default|GetCurrentQuest)) false false "(R=0.000000,G=0.660000,B=1.000000,A=1.000000)" 4.0))

(fn GetQuest
  (return (Variables|Default|GetHasQuest) (Variables|Default|GetCurrentQuest)))

(fn OnNewQuestCompleted
  (params (QuestDetails :type S%20Quest%20Details%20Structure))
  (if (== (Utilities|Struct|BreakS_QuestDetails QuestDetails) (Utilities|Struct|BreakS_QuestDetails (Variables|Default|GetCurrentQuest)))
    (Variables|Default|SetHasQuest false)
    (Variables|Default|SetCurrentQuest "")))