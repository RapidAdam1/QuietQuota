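; Quest manager Blueprint that runs an ordered list of quests, with one current quest tracked at a time.
; Initialize calls SetNewQuest, which spawns the next quest class as an actor, binds an event to its OnCompleted dispatcher and advances the index.
; Once the list is exhausted, it only reaches a completion PrintString with screen and log output disabled.
; GetTargets exposes the stored Targets.
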(event Custom|Initialize
  (CallFunction|SetNewQuest))

(fn ConstructionScript)

(fn GetTargets
  (return (Variables|Default|GetTargets)))

(fn SetNewQuest
  (if (< (Variables|Default|GetCurrentQuestIndex) (Utilities|Array|Length (Variables|Default|GetQuests)))
    (bind _returnvalue (Game|SpawnActorfromClass (Utilities|Array|Get(acopy) (Variables|Default|GetQuests) (Variables|Default|GetCurrentQuestIndex)) (Math|Transform|MakeTransform "0, 0, 0" "0, 0, 0" "1.000000,1.000000,1.000000") "AlwaysSpawn" "MultiplyWithRoot" 0 0))
    (Variables|Default|SetCurrentQuest _returnvalue)
    (EventDispatchers|BindEventtoOnCompleted (Variables|Default|GetCurrentQuest) (EventDispatchers|CreateEvent :!event SetNewQuest))
    (Math|Integer|IncrementInt (Variables|Default|GetCurrentQuestIndex))
    (else
      (Development|PrintString "Completed all quests" false false))))