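; AC_QuestTask is a quest component that holds one assigned task and reports when it completes.
; Assign stores the task details and quest reference, flags the task as assigned and broadcasts OnTaskAssigned.
; CheckCompleted verifies that the quest's current task ID matches the stored one, then broadcasts OnTaskCompleted, destroys the component and forces garbage collection.
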(fn Assign
  (params (TaskDetails :type S%20Quest%20Details%20Structure) (Quest :type BP%20Base%20Quest%20Object%20Reference))
  (Variables|Default|SetTaskDetails TaskDetails)
  (Variables|Default|SetQuestRef Quest)
  (Variables|Default|SetHasAssignedTask true)
  (Default|CallOnTaskAssigned (Variables|Default|GetTaskDetails)))

(fn CheckCompleted
  (if (Variables|Default|GetHasAssignedTask)
    (if (== (Utilities|Struct|BreakS_QuestDetails (Default|GetCurrentTaskDetails (Variables|Default|GetQuestRef))) (Utilities|Struct|BreakS_QuestDetails (Variables|Default|GetTaskDetails)))
      (Default|CallOnTaskCompleted (Variables|Default|GetTaskDetails))
      (Components|DestroyComponent)
      (Utilities|Platform|CollectGarbage))))