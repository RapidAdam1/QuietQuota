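; Quest task that sends the player back to the level's start by placing an objective end marker there.
; On initialize it spawns BP_ObjectiveEnd at the location of a PlayerStart and assigns the current task details and quest to its AC_QuestTask component.
; It also binds to that component's completion event; its OnTaskCompleted function prints the completed task's name once, guarded by a HasCompleted flag.
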(event EventInitialize
  (params (CurrentQuest :type BP%20Base%20Quest%20Object%20Reference))
  (|CallParentFunction CurrentQuest)
  (Variables|Default|SetCurrent%20Quest CurrentQuest)
  (bind _returnvalue (Actor|GetActorOfClass "/Script/Engine.PlayerStart"))
  (bind _returnvalue_2 (Game|SpawnActorfromClass "/Game/Core/AdvancedObjectives/BP_ObjectiveEnd.BP_ObjectiveEnd_C" (Math|Transform|MakeTransform (Transformation|GetActorLocation _returnvalue) "0, 0, 0" "1.000000,1.000000,1.000000") "Undefined" "MultiplyWithRoot" 0 0))
  (EventDispatchers|BindEventtoOnTaskCompleted (Actor|GetComponentbyClass _returnvalue_2 "/Game/Core/Quest_System/QuestsToDo/AC_QuestTask.AC_QuestTask_C") (EventDispatchers|CreateEvent :!event OnTaskCompleted))
  (Default|Assign (Actor|GetComponentbyClass _returnvalue_2 "/Game/Core/Quest_System/QuestsToDo/AC_QuestTask.AC_QuestTask_C") (Default|GetCurrentTaskDetails (Variables|Default|GetCurrent%20Quest)) (Variables|Default|GetCurrent%20Quest)))

(fn ConstructionScript)

(fn OnTaskCompleted
  (params (QuestDetails :type S%20Quest%20Details%20Structure))
  (if (not (Variables|Default|GetHasCompleted))
    (Development|PrintText (Utilities|Text|FormatText "Completed Quest Task: {name}" (Utilities|Struct|BreakS_QuestDetails QuestDetails)))
    (Variables|Default|SetHasCompleted true)))