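; BP_Quest_Task is a quest task in the quest system that tracks completion through its targets.
; On Initialize it runs the parent logic, then binds a delegate to the quest-completed event of each entry in Targets.
; OnTaskCompleted uses a HasCompleted flag to act only once, printing the completed task's item name and setting the flag, with no check that all targets are done.
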(event EventInitialize
  (params (CurrentQuest :type BP%20Base%20Quest%20Object%20Reference))
  (|CallParentFunction CurrentQuest)
  (for _array_element (Variables|Default|GetTargets)
    (EventDispatchers|BindEventtoOnQuestCompleted _array_element (EventDispatchers|CreateEvent :!event OnTaskCompleted))))

(fn ConstructionScript)

(fn OnTaskCompleted
  (params (QuestDetails :type S%20Quest%20Details%20Structure))
  (if (not (Variables|Default|GetHasCompleted))
    (Development|PrintText (Utilities|Text|FormatText "Completed Quest Task: {name}" (Utilities|Struct|BreakS_QuestDetails QuestDetails)))
    (Variables|Default|SetHasCompleted true)))