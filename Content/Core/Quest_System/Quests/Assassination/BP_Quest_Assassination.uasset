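; Assassination quest Blueprint that hands out randomized kill-target tasks from DT_QuestDetails_Assassination to AI characters.
; AssignRandomizedQuests picks a random row per target and assigns it through that actor's AC_QuestTask component.
; SetNextTask extends the parent by printing the task's clue on screen.
; Target gathering, informant assignment and completion binding are disconnected, so BeginPlay, LoadAssisnation and InitializeTargets currently do nothing.
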(event Custom|LoadAssisnation
  (params (QuestDetails :type S%20Quest%20Details%20Structure)))

(event EventBeginPlay)

(fn ConstructionScript)

(fn SetNextTask
  (params (QuestDetails :type S%20Quest%20Details%20Structure))
  (|CallParentFunction QuestDetails)
  (Development|PrintString (.Clue (Utilities|Struct|BreakS_QuestDetails QuestDetails)) true true "(R=1.000000,G=0.000000,B=0.050806,A=1.000000)" 1e+01))

(fn AssignRandomizedQuests
  (params (TargetItems :type Array%20of%20Actor%20Object%20References) (QuestNames :type Array%20of%20Names))
  ;[1 1 1] Get Randomized Quests
  (bind _randomizednames (CallFunction|GetRandomizedRowNames QuestNames (Utilities|Array|Length TargetItems)))
  (Variables|Default|SetDTQuestNames _randomizednames)
  (for (_array_element _array_index) TargetItems
    (LocalVariables|SetL_CurrentElement _array_element)
    (LocalVariables|SetL_CurrentIndex _array_index)
    (bind _returnvalue (Utilities|GetDataTableRow "/Game/Core/Quest_System/Quests/Assassination/DT_QuestDetails_Assassination.DT_QuestDetails_Assassination" (Utilities|Array|Get(acopy) (Variables|Default|GetDTQuestNames) (LocalVariables|GetL_CurrentIndex)))
      (:then
        (Utilities|Array|Add (LocalVariables|GetL_QuestDetail) _returnvalue)
        (Default|Assign (Actor|GetComponentbyClass (LocalVariables|GetL_CurrentElement) "/Game/Core/Quest_System/QuestsToDo/AC_QuestTask.AC_QuestTask_C") _returnvalue self))))
  (return (LocalVariables|GetL_QuestDetail)))

(fn GetTargets
  (return (Variables|Default|GetTargets)))