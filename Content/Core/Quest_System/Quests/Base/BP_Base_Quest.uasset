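; Base quest Blueprint that runs a list of task classes in order, one active task at a time.
; SetNextTask destroys the current task and forces garbage collection, then spawns the next task, binds its completion event, stores the quest details and initializes it with the quest.
; Helpers expose the current task details and draw a requested number of random row names without repeating a pick.
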(event EventBeginPlay)

(fn ConstructionScript)

(fn SetNextTask
  (params (QuestDetails :type S%20Quest%20Details%20Structure))
  (bind _currenttaskindex (Variables|Default|GetCurrentTaskIndex))
  (Development|PrintString (Utilities|String|ToString(Integer) _currenttaskindex))
  (if (< _currenttaskindex (Utilities|Array|Length (Variables|Default|GetTasks)))
    (Utilities|FlowControl|Sequence
      (:then_0
        (Utilities|IsValid (Variables|Default|GetCurrentTask)
          (:Is%20Valid
            (Actor|DestroyActor (Variables|Default|GetCurrentTask))
            (Utilities|Platform|CollectGarbage))))
      (:then_1
        (bind _returnvalue (Game|SpawnActorfromClass (Utilities|Array|Get(acopy) (Variables|Default|GetTasks) (Variables|Default|GetCurrentTaskIndex)) (Math|Transform|MakeTransform "0, 0, 0" "0, 0, 0" "1.000000,1.000000,1.000000") "AlwaysSpawn" "MultiplyWithRoot" 0 0))
        (bind _output_get (Variables|Default|SetCurrentTask _returnvalue))
        (EventDispatchers|BindEventtoOnCompleted _output_get (EventDispatchers|CreateEvent :!event SetNextTask))
        (Variables|Default|SetCurrentTaskDetails QuestDetails)
        (Math|Integer|IncrementInt (Variables|Default|GetCurrentTaskIndex)
          (:%20%20
            (Default|Initialize (Variables|Default|GetCurrentTask) self)))))
    (else
      (Development|PrintString "Completed all tasks"))))

(fn GetCurrentTaskDetails
  (return (Variables|Default|GetCurrentTaskDetails)))

(fn GetRandomizedRowNames
  (params (RowNames :type Array%20of%20Names) (TargetLength :type Integer))
  (LocalVariables|SetL_RawNames RowNames)
  (LocalVariables|SetL_MinLength (- (Utilities|Array|Length (LocalVariables|GetL_RawNames)) TargetLength))
  (while (> (Utilities|Array|Length (LocalVariables|GetL_RawNames)) (LocalVariables|GetL_MinLength))
    (LocalVariables|SetL_CurrentName (.OutItem (Utilities|Array|Random (LocalVariables|GetL_RawNames))))
    (Utilities|Array|Add (LocalVariables|GetL_RandomizedNames) (LocalVariables|GetL_CurrentName))
    (Utilities|Array|RemoveItem (LocalVariables|GetL_RawNames) (LocalVariables|GetL_CurrentName)))
  (return (LocalVariables|GetL_RandomizedNames)))