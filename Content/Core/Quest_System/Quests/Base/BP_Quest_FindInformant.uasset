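; BP_Quest_FindInformant is a quest Blueprint in the quest system, built around the informant actor in the level.
; On InitializeQuest it stores the task details and finds BP_Level_Informant by class.
; It assigns the details and itself to that actor's AC_QuestTask component, then binds to the component's task-completed dispatcher.
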(event EventBeginPlay
  (|CallParentFunction))

(event EventInitializeQuest
  (params (TaskDetails :type S%20Quest%20Details%20Structure))
  (bind _output_get (Variables|Default|SetTask%20Details TaskDetails))
  (bind _returnvalue (Actor|GetActorOfClass "/Game/Core/Interaction_System/BP_Level_Informant.BP_Level_Informant_C"))
  (Default|Assign (Actor|GetComponentbyClass _returnvalue "/Game/Core/Quest_System/QuestsToDo/AC_QuestTask.AC_QuestTask_C") _output_get self)
  (EventDispatchers|BindEventtoOnTaskCompleted (Actor|GetComponentbyClass _returnvalue "/Game/Core/Quest_System/QuestsToDo/AC_QuestTask.AC_QuestTask_C") (EventDispatchers|CreateEvent :!event SetNextTask)))

(fn ConstructionScript
  (|CallParentFunction))