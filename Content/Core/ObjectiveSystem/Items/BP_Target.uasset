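; BP_Target is a killable objective item in the objective system, shown as a Paper2D flipbook.
; SetDetails extends the parent setup by tinting the flipbook with the selected quest's item colour.
; CanKill shows or hides the kill prompt widget.
; OnKill stores the killer if it is a BP_PlayerCharacter, then has the ACTaskToDo task, when valid, check for completion.
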(event EventBeginPlay
  (|CallParentFunction))

(event EventOnKill
  (params (Killer :type Actor%20Object%20Reference))
  (bind _asbp_player_character (Utilities|Casting|CastToBP_PlayerCharacter Killer))
  (Variables|Default|SetL_CharRef _asbp_player_character)
  (Utilities|IsValid (Variables|Default|GetAC_TaskToDo)
    (:Is%20Valid
      (Default|CheckCompleted (Variables|Default|GetAC_TaskToDo)))))

(event EventCanKill
  (params (CanKill :type Boolean))
  (Development|SetHiddeninGame (Variables|Default|GetBPW_Prompt_Kill) (not CanKill) false))

(fn ConstructionScript
  (|CallParentFunction))

(fn SetDetails
  (params (SelectedQuest :type S%20Quest%20Details%20Structure))
  (|CallParentFunction SelectedQuest)
  (Sprite|SetSpriteColor (Variables|Default|GetPaperFlipbook) (Utilities|Struct|BreakS_QuestDetails SelectedQuest)))