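; Key pickup that the player collects by walking into it, granting a key and enabling lockpicking.
; On BeginPlay, a half-speed timeline lerps the sparkle particle between its starting position and a point slightly above it.
; When BP_PlayerCharacter overlaps the box, it plays a 2D collect sound, sets CanLockpick, stops the animation, increments the key count through AlterKeys and destroys itself.
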(event OnComponentBeginOverlap(Box)
  (params (OverlappedComponent :type Primitive%20Component%20Object%20Reference) (OtherActor :type Actor%20Object%20Reference) (OtherComp :type Primitive%20Component%20Object%20Reference) (OtherBodyIndex :type Integer) (bFromSweep :type Boolean) (SweepResult :type Hit%20Result%20Structure%20%28by%20ref%29))
  (bind _asbp_player_character (Utilities|Casting|CastToBP_PlayerCharacter OtherActor))
  (bind _output_get (Variables|Default|SetPlayer _asbp_player_character))
  (Audio|PlaySound2D "/Game/UI/UI_Audio/CollectValuable_Cue.CollectValuable_Cue" 1.0 1.0 0.0 0 0)
  (Variables|/Game/Core/PlayerCharacter/BP_PlayerCharacter.BP_PlayerCharacter_C|SetCanLockpick _output_get true)
  (Audio|Components|Audio|Stop (Variables|Default|GetTimeline_Idle))
  (Transformation|SetRelativeLocation (Variables|Default|GetPS_Sparkle) "0, 0, 0" false false)
  (Default|AlterKeys (Variables|Default|GetPlayer) 1)
  (Actor|DestroyActor))

(event EventBeginPlay
  (|CallParentFunction)
  (Variables|Default|SetPSStartLoc (Variables|/Script/Engine.SceneComponent|GetRelativeLocation (Variables|Default|GetPS_Sparkle)))
  (Variables|Default|SetPSEndLoc (+ (Variables|Default|GetPSStartLoc) "0.000000,0.000000,50.000000"))
  (Components|Timeline|SetPlayRate (Variables|Default|GetTimeline_Idle) 0.5)
  (bind _lerp (Timeline|Timeline_Idle Play)
    (:Update
      (Transformation|SetRelativeLocation (Variables|Default|GetPS_Sparkle) (Math|Vector|Lerp(Vector) (Variables|Default|GetPSStartLoc) (Variables|Default|GetPSEndLoc) _lerp) false false))))

(event Collision|EventActorBeginOverlap
  (params (OtherActor :type Actor%20Object%20Reference))
  (|CallParentFunction OtherActor) ; This node is disabled and will not be called.\nDrag off pins to build functionality.
)

(event EventTick
  (params (DeltaSeconds :type Float%20%28single-precision%29))
  (|CallParentFunction DeltaSeconds) ; This node is disabled and will not be called.\nDrag off pins to build functionality.
)

(fn ConstructionScript
  (|CallParentFunction))