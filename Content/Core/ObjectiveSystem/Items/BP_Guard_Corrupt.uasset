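; BP_Guard_Corrupt is an objective-system actor, by name a corrupt guard, that serves as a proximity trigger for a quest task.
; When the player character overlaps its Box, it asks its quest task component to check completion.
; The completion handler passes the task's clue to a Print String with screen and log output off, so nothing shows.
; SetDetails and the construction script only call the parent.
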(event OnComponentBeginOverlap(Box)
  (params (OverlappedComponent :type Primitive%20Component%20Object%20Reference) (OtherActor :type Actor%20Object%20Reference) (OtherComp :type Primitive%20Component%20Object%20Reference) (OtherBodyIndex :type Integer) (bFromSweep :type Boolean) (SweepResult :type Hit%20Result%20Structure%20%28by%20ref%29))
  (Utilities|Casting|CastToBP_PlayerCharacter OtherActor)
  (Utilities|IsValid (Variables|Default|GetAC_QuestTask)
    (:Is%20Valid
      (Default|CheckCompleted (Variables|Default|GetAC_QuestTask)))))

(event OnTaskCompleted(AC_QuestTask)
  (params (TaskDetails :type S%20Quest%20Details%20Structure))
  (Development|PrintString (.Clue (Utilities|Struct|BreakS_QuestDetails TaskDetails)) false false "(R=0.000000,G=0.660000,B=1.000000,A=1.000000)" 1e+01))

(event EventBeginPlay
  (|CallParentFunction) ; This node is disabled and will not be called.\nDrag off pins to build functionality.
)

(event Collision|EventActorBeginOverlap
  (params (OtherActor :type Actor%20Object%20Reference))
  (|CallParentFunction OtherActor) ; This node is disabled and will not be called.\nDrag off pins to build functionality.
)

(event EventTick
  (params (DeltaSeconds :type Float%20%28single-precision%29))
  (|CallParentFunction DeltaSeconds) ; This node is disabled and will not be called.\nDrag off pins to build functionality.
)

(fn ConstructionScript
  (|CallParentFunction))

(fn SetDetails
  (params (SelectedQuest :type S%20Quest%20Details%20Structure))
  (|CallParentFunction SelectedQuest))