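; Player character component that detects the nearest interactable or killable actor for the objective system.
; A looping timer drives detection: a sphere overlap sorted by distance selects the first actor implementing the kill or interact interface, with kill checked first per actor.
; The target is told whether action is possible: interaction needs range, kills also need the player within an angle behind it.
; OnPerformAction sends both interact and kill messages to that target.
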(event Custom|StartTargetDetection
  (Utilities|Time|SetTimerbyEvent (EventDispatchers|CreateEvent :!event TargetDetection) (Variables|General|GetCheckRate) true))

(event EventBeginPlay
  (bind _asbp_player_character (Utilities|Casting|CastToBP_PlayerCharacter (Components|GetOwner)))
  (Variables|General|SetPlayerRef _asbp_player_character)
  (CallFunction|StartTargetDetection))

(fn TargetDetection
  (bind (_outactors _returnvalue) (Collision|SphereOverlapActors (Transformation|GetActorLocation (Variables|General|GetPlayerRef)) (Variables|General|GetTraceDistance) (Utilities|Array|MakeArray "ObjectTypeQuery3" "ObjectTypeQuery1" "ObjectTypeQuery2" "ObjectTypeQuery4") 0 (Utilities|Array|MakeArray (Variables|General|GetPlayerRef))))
  (if _returnvalue
    (bind _distancesortedarray (CallFunction|OrderbyClosestDistance _outactors (Transformation|GetActorLocation (Variables|General|GetPlayerRef))))
    (for _array_element _distancesortedarray
      (bind _output_get (LocalVariables|SetL_TargetActor _array_element))
      (Utilities|FlowControl|Sequence
        (:then_0
          (if (Utilities|DoesObjectImplementInterface _output_get "/Game/Core/ObjectiveSystem/BPI_Kill_Item.BPI_Kill_Item_C")
            (CallFunction|NullTarget)
            (Variables|General|SetDetectedTarget (LocalVariables|GetL_TargetActor))
            (bind _performaction (CallFunction|CanDoAction (Variables|Interact|GetInteractRadius) (Variables|Interact|GetInteractDistance) (Transformation|GetActorTransform (LocalVariables|GetL_TargetActor))))
            (Class|BPIKillItem|CanKill(Message) (Variables|General|GetDetectedTarget) _performaction)
            (return)))
        (:then_1
          (if (Utilities|DoesObjectImplementInterface _output_get "/Game/Core/DragonQuest/BPI_InteractWith.BPI_InteractWith_C")
            (CallFunction|NullTarget)
            (Variables|General|SetDetectedTarget (LocalVariables|GetL_TargetActor))
            (Class|BPIInteractwith|CanInteract(Message) (LocalVariables|GetL_TargetActor) (<= (Math|Vector|Distance(Vector) (Transformation|GetActorLocation (LocalVariables|GetL_TargetActor)) (Transformation|GetActorLocation (Variables|General|GetPlayerRef))) (Variables|Interact|GetInteractDistance)))
            (return)))))
    (else
      (CallFunction|NullTarget))))

(fn OnPerformAction
  (Utilities|IsValid (Variables|General|GetDetectedTarget)
    (:Is%20Valid
      (Class|BPIInteractwith|OnInteract(Message) (Variables|General|GetDetectedTarget) (Variables|General|GetPlayerRef))
      (Class|BPIKillItem|OnKill(Message) (Variables|General|GetDetectedTarget) (Variables|General|GetPlayerRef)))))

(fn CanDoAction
  (params (TestAngle :type Float%20%28double-precision%29) (TestDistance :type Float%20%28double-precision%29) (TestTransform :type Transform))
  (bind _playerref (Variables|General|GetPlayerRef))
  (bind _rotation (Math|Transform|BreakTransform TestTransform))
  (bind _location (Math|Transform|BreakTransform TestTransform))
  (bind _returnvalue (Transformation|GetActorLocation _playerref))
  (bind _returnvalue_2 (Math|Vector|GetForwardVector _rotation))
  (bind _returnvalue_3 (Math|Vector|GetUnitDirection(Vector) _location _returnvalue))
  (bind _returnvalue_4 (Math|Vector|NegateVector _returnvalue_2))
  (bind (_x _y) (Class|KismetMathLibrary|BreakVector3f _returnvalue_3))
  (bind (_x_2 _y_2) (Class|KismetMathLibrary|BreakVector3f _returnvalue_4))
  (return (and (<= (Class|KismetMathLibrary|DegAcos (Math|Vector2D|DotProduct(2D) (Math|Vector2D|MakeVector2D _x _y) (Math|Vector2D|MakeVector2D _x_2 _y_2))) TestAngle) (<= (Math|Vector|Distance(Vector) (.Location (Math|Transform|BreakTransform TestTransform)) (Transformation|GetActorLocation (Variables|General|GetPlayerRef))) TestDistance))))

(fn OrderbyClosestDistance
  (params (UnsortedArray :type Array%20of%20Actor%20Object%20References) (CompareLocation :type Vector))
  (LocalVariables|SetL_RawArray UnsortedArray)
  (while (> (Utilities|Array|Length (LocalVariables|GetL_RawArray)) 0)
    (LocalVariables|SetL_CompareDistance 1e+10)
    (for _array_element (LocalVariables|GetL_RawArray)
      (if (< (Class|KismetMathLibrary|VectorDistance2DSquared (Transformation|GetActorLocation _array_element) CompareLocation) (LocalVariables|GetL_CompareDistance))
        (LocalVariables|SetL_LowestDistance _array_element)
        (LocalVariables|SetL_CompareDistance (Class|KismetMathLibrary|VectorDistance2DSquared (Transformation|GetActorLocation _array_element) CompareLocation))))
    (Utilities|Array|Add (LocalVariables|GetL_SortedArray) (LocalVariables|GetL_LowestDistance))
    (Utilities|Array|Add (LocalVariables|GetL_TestLengths) (LocalVariables|GetL_CompareDistance))
    (Utilities|Array|RemoveItem (LocalVariables|GetL_RawArray) (LocalVariables|GetL_LowestDistance)))
  (return (LocalVariables|GetL_SortedArray)))

(fn NullTarget
  (Utilities|IsValid (Variables|General|GetDetectedTarget)
    (:Is%20Valid
      (Class|BPIInteractwith|CanInteract(Message) (Variables|General|GetDetectedTarget) false)
      (Class|BPIKillItem|CanKill(Message) (Variables|General|GetDetectedTarget) false)
      (Variables|General|SetDetectedTarget 0))))