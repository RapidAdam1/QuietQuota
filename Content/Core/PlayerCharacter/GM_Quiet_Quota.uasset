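; GM_Quiet_Quota is the Quiet Quota game mode, handling level music and quest start-up.
; The LevelTheme audio component fades in at BeginPlay and, whenever a track finishes, alternates between LevelMusic_Cue and AmbientMusic_Cue.
; A FadeOut event fades the music out, and GenerateQuests spawns BP_Quest_Spawner and calls StartQuests on it.
; An unconnected objective Initialise call is left unused in the graph.
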(event OnAudioFinished(LevelTheme)
  (bind _leveltheme (Variables|Default|GetLevelTheme))
  (bind _leveltheme_2 (Variables|Default|GetLevelTheme))
  (if (== (Variables|/Script/Engine.AudioComponent|GetSound (Variables|Default|GetLevelTheme)) "/Game/UI/UI_Audio/LevelMusic_Cue.LevelMusic_Cue")
    (Audio|Components|Audio|SetSound _leveltheme_2 "/Game/UI/UI_Audio/AmbientMusic_Cue.AmbientMusic_Cue")
    (Audio|Components|Audio|FadeIn _leveltheme_2 0.0 1.0 0.0 "Linear" :!class /Script/Engine.AudioComponent)
    (else
      (Audio|Components|Audio|SetSound _leveltheme "/Game/UI/UI_Audio/LevelMusic_Cue.LevelMusic_Cue")
      (Audio|Components|Audio|FadeIn _leveltheme 0.0 1.0 0.0 "Linear" :!class /Script/Engine.AudioComponent))))

(event Custom|Generate%20Quests
  (bind _returnvalue (Game|SpawnActorfromClass "/Game/Core/DragonQuest/BP_Quest_Spawner.BP_Quest_Spawner_C" (Math|Transform|MakeTransform "0, 0, 0" "0, 0, 0" "1.000000,1.000000,1.000000") "AlwaysSpawn" "MultiplyWithRoot" 0 0))
  (Default|StartQuests _returnvalue))

(event Custom|FadeOut
  (Audio|Components|Audio|FadeOut (Variables|Default|GetLevelTheme) 1.0 0.0 "Linear" :!class /Script/Engine.AudioComponent))

(event EventBeginPlay
  (Audio|Components|Audio|FadeIn (Variables|Default|GetLevelTheme) 0.0 1.0 0.0 "Linear" :!class /Script/Engine.AudioComponent))

(fn ConstructionScript)