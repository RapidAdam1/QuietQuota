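; BP_FORANDREW is an unfinished prototype of item hotkeys 1–5 for the player character.
; Key 3, when the potion count is zero or below, sets a translucent sprite material and clears CanBeSeen until a timer restores it; its opacity material instances are never assigned.
; Key 5, under a similar count check, sphere-traces pawns and casts to AI_Character without further action.
; Key, lockpick, smoke bomb and GOTOSLEEP logic are empty.
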(event Custom|InvisTimer
  (bind _returnvalue (Rendering|Material|CreateDynamicMaterialInstance (Variables|Default|GetTranslucentSpriteMat) "Opacity" "None" :!class /Script/Engine.KismetMaterialLibrary))
  (Rendering|Material|SetScalarParameterValue _returnvalue "Opacity" 1.0 :!class /Script/Engine.MaterialInstanceDynamic)
  (Variables|Default|SetCanBeSeen? true))

(event Custom|GOTOSLEEP)

(event Input|KeyboardEvents|1
  (params (Key :type Key%20Structure :default "None"))
  (:Pressed
    (if (<= (Variables|Default|GetNumberOfKeys) 0)
      _)))

(event Input|KeyboardEvents|2
  (params (Key :type Key%20Structure :default "None"))
  (:Pressed
    (if (<= (Variables|Default|GetNumberOfLockpicks) 0)
      _)))

(event Input|KeyboardEvents|3
  (params (Key :type Key%20Structure :default "None"))
  (:Pressed
    (if (<= (Variables|Default|GetNumberOfInvisPotions) 0)
      (bind _returnvalue (Actor|GetActorOfClass "/Game/Core/PlayerCharacter/BP_PlayerCharacter.BP_PlayerCharacter_C"))
      (Rendering|Material|SetMaterial (Variables|/Game/Core/PlayerCharacter/BP_PlayerCharacter.BP_PlayerCharacter_C|GetPaperFlipbook _returnvalue) 0 (Variables|Default|GetTranslucentSpriteMat))
      (bind _returnvalue_2 (Rendering|Material|CreateDynamicMaterialInstance (Variables|Default|GetTranslucentSpriteMat) "Opacity" "None" :!class /Script/Engine.KismetMaterialLibrary))
      (Rendering|Material|SetScalarParameterValue _returnvalue_2 "Opacity" 0.1 :!class /Script/Engine.MaterialInstanceDynamic)
      (Variables|Default|SetCanBeSeen? false)
      (Utilities|Time|SetTimerbyEvent (delegate Custom|InvisTimer) 3e+01))))

(event Input|KeyboardEvents|4
  (params (Key :type Key%20Structure :default "None"))
  (:Pressed
    (if (<= (Variables|Default|GetNumberOfSmokeBombs) 0)
      _)))

(event Input|KeyboardEvents|5
  (params (Key :type Key%20Structure :default "None"))
  (bind _self self)
  (bind _returnvalue (Transformation|GetActorLocation _self))
  (:Pressed
    (if (<= (Variables|Default|GetNumberOfSleepPowder) 0)
      (bind _outhits (Collision|MultiSphereTraceForObjects _returnvalue _returnvalue 3e+02 (Utilities|Array|MakeArray "ObjectTypeQuery3") false 0 "None"))
      (for _array_element _outhits
        (Utilities|Casting|CastToAI_Character (.HitActor (Collision|BreakHitResult _array_element)))))))

(fn ConstructionScript)