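; Interactable door that opens once, optionally locked with padlock sprites and opened by spending a player key or, failing that, a lockpick.
; On interact, a dot product against the door's right vector picks the swing direction from the player's side.
; A timeline then rotates the pivot, plays a sound and finally disables detection collision.
; The interact prompt on a locked door shows only when the player holds a key or lockpick.
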(event Custom|Unlock%20Door
  ;[0 0 0] Unlock Door
  (Utilities|FlowControl|DoOnce false
    (:Completed
      (Variables|Default|SetIsOpen true)
      (Audio|PlaySound2D "/Game/UI/UI_Audio/OpenDoorChest_Cue.OpenDoorChest_Cue" 1.0 1.0 0.0 0 0)
      (Development|SetHiddeninGame (Variables|Default|GetBPW_InteractPrompt) true false)
      (bind _newtrack_0 (Timeline|Timeline_DoorOpen PlayFromStart)
        (:Update
          (Transformation|SetRelativeRotation (Variables|Default|GetPivot) (Math|Rotator|Lerp(Rotator) (Variables|Default|GetPivotDefaultRotation) (Variables|Default|GetTarget%20Rotation) _newtrack_0 true) false false))
        (:Finished
          (Collision|SetCollisionEnabled (Variables|Default|GetCollision_PlayerDetect) "NoCollision"))))))

(event Custom|LockDoor
  ;[0 0 0] Lock Door
)

(event EventCanInteract
  (params (CanInteract :type Boolean))
  (bind _player_character (Variables|Default|GetPlayer%20Character))
  (bind _player_character_2 (Variables|Default|GetPlayer%20Character))
  (bind _keysvalue (Variables|/Game/Core/PlayerCharacter/BP_PlayerCharacter.BP_PlayerCharacter_C|GetKeysValue _player_character_2))
  (bind _lockpicksvalue (Variables|/Game/Core/PlayerCharacter/BP_PlayerCharacter.BP_PlayerCharacter_C|GetLockPicksValue _player_character))
  (bind _returnvalue (> _lockpicksvalue 0))
  (bind _returnvalue_2 (> _keysvalue 0))
  (bind _returnvalue_3 (or _returnvalue_2 _returnvalue))
  (if CanInteract
    (if (not (Variables|Default|GetIsOpen))
      (if (Variables|Default|GetIsLocked?)
        (Development|SetHiddeninGame (Variables|Default|GetBPW_InteractPrompt) (not _returnvalue_3) false)
        (Development|PrintString (Utilities|String|ToString(Boolean) _returnvalue_3) false false)
        (else
          (Development|SetHiddeninGame (Variables|Default|GetBPW_InteractPrompt) (not CanInteract) false :!label _label))))
    (else
      (goto _label))))

(event Collision|EventActorBeginOverlap
  (params (OtherActor :type Actor%20Object%20Reference)))

(event EventOnInteract
  (params (PlayerRef :type BP%20Player%20Character%20Object%20Reference))
  ;[0 0 0] Begin Overlap
  (if (Variables|Default|GetIsLocked?)
    (if (> (Variables|/Game/Core/PlayerCharacter/BP_PlayerCharacter.BP_PlayerCharacter_C|GetKeysValue (Variables|Default|GetPlayer%20Character)) 0)
      (Default|AlterKeys (Variables|Default|GetPlayer%20Character) -1)
      (Variables|Default|SetTarget%20Rotation (Math|Rotator|SelectRotator "0.000000,90.000000,0.000000" "0.000000,-90.000000,0.000000" (> (Math|Vector2D|DotProduct(2D) (Math|Conversions|ToVector2D(Vector) (Math|Vector|GetUnitDirection(Vector) (Transformation|GetActorLocation PlayerRef) (Transformation|GetActorLocation))) (Math|Conversions|ToVector2D(Vector) (Transformation|GetActorRightVector))) 0.0)) :!label _label)
      (CallFunction|UnlockDoor)
      (Utilities|FlowControl|DoOnce false
        (:Completed
          (Components|DestroyComponent (Variables|Default|GetPadlock8x8_Sprite))))
      (elif (> (Variables|/Game/Core/PlayerCharacter/BP_PlayerCharacter.BP_PlayerCharacter_C|GetLockPicksValue (Variables|Default|GetPlayer%20Character)) 0)
        (Default|AlterLockpicks (Variables|Default|GetPlayer%20Character) -1)
        (goto _label)))
    (else
      (goto _label))))

(event EventBeginPlay
  ;[0 0 0] Begin Play
  (Utilities|FlowControl|Sequence
    (:then_0
      (bind _returnvalue (Actor|GetActorOfClass "/Game/Core/PlayerCharacter/BP_PlayerCharacter.BP_PlayerCharacter_C"))
      (Variables|Default|SetPlayer%20Character _returnvalue)
      (CallFunction|LockDoor)
      (Variables|Default|SetPivotDefaultRotation (Variables|/Script/Engine.SceneComponent|GetRelativeRotation (Variables|Default|GetPivot)))
      (Components|Timeline|SetPlayRate (Variables|Default|GetTimeline_DoorOpen) (Variables|Default|GetDoorSpeed)))
    (:then_1
      (if (not (Variables|Default|GetIsLocked?))
        (Development|SetHiddeninGame (Variables|Default|GetPadlock8x8_Sprite1) true false)))))

(fn ConstructionScript)

(fn ToggleDoor
  (params (Can%20LockPick? :type Boolean))
  ;[0 0 0] Toggle Door
  (if Can%20LockPick?
    (CallFunction|UnlockDoor)
    (else
      (CallFunction|LockDoor))))