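; Dialogue component that gives an AI character floating barks for idle, player-detected and player-lost states.
; It spawns a following widget actor, broadcasts lines to it, and destroys it when the AI is killed.
; Each state draws random conversations from its DataTable using a shrinking, refillable row pool.
; Timers pace lines by text length and conversations by random delay; detection changes interrupt both, and lost-player plays one line before reverting to idle.
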(event Custom|CallToUpdateDialogue
  ;[0 0 0] Play Dialogue
  (CallFunction|PickRandomConversation (Variables|Default|GetCurrentState)))

(event Custom|InitializeWithController
  (params (ControllerRef :type Enemy%20Controller%20Base%20Object%20Reference))
  ;[0 0 0] Initialize Dialogue
  (EventDispatchers|BindEventtoOnDetectedPlayer ControllerRef (EventDispatchers|CreateEvent :!event Custom|OnPlayerDetected))
  (CallFunction|CreateDialogueWidget)
  (Utilities|FlowControl|Sequence
    (:then_0
      (bind _asai_character (Utilities|Casting|CastToAI_Character (Components|GetOwner)))
      (EventDispatchers|BindEventtoOnKilledAI _asai_character (EventDispatchers|CreateEvent :!event Custom|OnAIKilled)))
    (:then_1
      (Utilities|Array|Clear (Variables|Dialogue|GetAllRowNames))
      (Utilities|Array|Clear (Variables|Dialogue|GetCurrentRowNames))
      (Variables|Default|SetCurrentState "NewEnumerator3")
      (CallFunction|PickRandomConversation "NewEnumerator0"))))

(event Custom|OnPlayerDetected
  (params (HasDetected :type Boolean))
  ;[1 1 1] New Player Detected State
  (Utilities|Time|ClearandInvalidateTimerbyHandle (Variables|Autoplay|GetDialogueHandle))
  (Utilities|Time|ClearandInvalidateTimerbyHandle (Variables|Default|GetConvoHandle))
  (if HasDetected
    (CallFunction|PickRandomConversation "NewEnumerator1")
    (else
      (CallFunction|PickRandomConversation "NewEnumerator2"))))

(event Custom|Play%20Dialogue
  (bind _currentdialogue (Variables|Dialogue|GetCurrentDialogue))
  (bind _returnvalue (Utilities|Array|Length _currentdialogue))
  (bind _returnvalue_2 (- _returnvalue 1))
  ;[0 0 0] Play Dialogue
  (if (<= (Variables|Dialogue|GetDialogue%20Index) (Utilities|Select :Index (Variables|Default|GetCurrentState) :NewEnumerator3 _returnvalue_2 :NewEnumerator0 _returnvalue_2 :NewEnumerator1 _returnvalue_2 :NewEnumerator2 0))
    (Default|CallOnDialogueUpdated (Utilities|Array|Get(acopy) (Variables|Dialogue|GetCurrentDialogue) (Variables|Dialogue|GetDialogue%20Index)))
    (Math|Integer|IncrementInt (Variables|Dialogue|GetDialogue%20Index)
      (:%20%20
        (bind _returnvalue_3 (Utilities|Time|SetTimerbyEvent (EventDispatchers|CreateEvent :!event Custom|Play%20Dialogue) (CallFunction|GetDialoguePlayTime (Utilities|String|ToString(Text) (Utilities|Array|Get(acopy) (Variables|Dialogue|GetCurrentDialogue) (Variables|Dialogue|GetDialogue%20Index))))))
        (Variables|Autoplay|SetDialogueHandle _returnvalue_3)))
    (else
      (Default|CallOnDialogueEnded)
      (bind _returnvalue_4 (Utilities|Time|SetTimerbyEvent (delegate Custom|CallToUpdateDialogue) (Math|Random|RandomFloatinRangefromStream (Math|Random|MakeRandomStream (Math|Random|RandomIntegerinRange 0 100)) (Variables|Autoplay|GetMinIntervalDelay) (Variables|Autoplay|GetMaxIntervalDelay))))
      (Variables|Default|SetConvoHandle _returnvalue_4))))

(event Custom|OnAIKilled
  ;[1 1 1] On AI Killed
  (Actor|DestroyActor (Variables|Default|GetDialogueWidget)))

(event Custom|Pick%20Random%20Conversation
  (params (NewDialogueState :type EDialogueState%20Enum :default "NewEnumerator3"))
  ;[0 0 0] Pick Random Conversation
  (Variables|Dialogue|SetDialogue%20Index 0)
  (bind _newdialogue (CallFunction|GetNewDialogue NewDialogueState))
  (Variables|Dialogue|SetCurrentDialogue (.dialogue _newdialogue))
  (CallFunction|PlayDialogue self))

(fn GetNewDialogue
  (params (RequestedState :type EDialogueState%20Enum :default "NewEnumerator3"))
  (LocalVariables|SetL_NewState RequestedState)
  (Utilities|FlowControl|Sequence
    (:then_0
      (Utilities|FlowControl|Sequence
        (:then_0
          ;[1 1 1] Ensures Lost Player Only Lasts one step
          (if (Utilities|Enum|Equal(Enum) (Variables|Default|GetCurrentState) "NewEnumerator2")
            (LocalVariables|SetL_NewState "NewEnumerator0")))
        (:then_1
          ;[1 1 1] Update Row Names if Dialogue State has changed
          (if (Utilities|Enum|NotEqual(Enum) (Variables|Default|GetCurrentState) (LocalVariables|GetL_NewState))
            (bind _output_get (Variables|Dialogue|SetCurrentDT (Utilities|Select :Index (LocalVariables|GetL_NewState) :NewEnumerator3 "/Game/Core/Dialogue/Datatables/DT_Dialogue_Idle.DT_Dialogue_Idle" :NewEnumerator0 "/Game/Core/Dialogue/Datatables/DT_Dialogue_Idle.DT_Dialogue_Idle" :NewEnumerator1 "/Game/Core/Dialogue/Datatables/DT_Dialogue_PlayerDetected.DT_Dialogue_PlayerDetected" :NewEnumerator2 "/Game/Core/Dialogue/Datatables/DT_Dialogue_PlayerLost.DT_Dialogue_PlayerLost")))
            (bind _outrownames (DataTable|GetDataTableRowNames _output_get))
            (bind _output_get_2 (Variables|Dialogue|SetAllRowNames _outrownames))
            (Variables|Dialogue|SetCurrentRowNames _output_get_2)
            (Variables|Default|SetCurrentState (LocalVariables|GetL_NewState))))))
    (:then_1
      ;[1 1 1] If no Current Row names left, then reset them back to all selection
      (if (<= (Utilities|Array|Length (Variables|Dialogue|GetCurrentRowNames)) 0)
        (Utilities|Array|Shuffle (Variables|Dialogue|GetAllRowNames))
        (Variables|Dialogue|SetCurrentRowNames (Variables|Dialogue|GetAllRowNames))))
    (:then_2
      ;[1 1 1] Get Random Dialogue then remove from current names
      (bind _returnvalue (Utilities|GetDataTableRow (Variables|Dialogue|GetCurrentDT) (Utilities|Array|Get(acopy) (Variables|Dialogue|GetCurrentRowNames) (Math|Random|RandomIntegerinRangefromStream (Math|Random|MakeRandomStream (Math|Random|RandomIntegerinRange 0 100)) 0 (- (Utilities|Array|Length (Variables|Dialogue|GetCurrentRowNames)) 1))))
        (:then
          (Utilities|Array|RemoveItem (Variables|Dialogue|GetCurrentRowNames) (Utilities|Array|Get(acopy) (Variables|Dialogue|GetCurrentRowNames) (Math|Random|RandomIntegerinRangefromStream (Math|Random|MakeRandomStream (Math|Random|RandomIntegerinRange 0 100)) 0 (- (Utilities|Array|Length (Variables|Dialogue|GetCurrentRowNames)) 1))))
          (return _returnvalue))))))

(fn CreateDialogueWidget
  (bind _returnvalue (Game|SpawnActorfromClass "/Game/Core/Dialogue/BP_DialogueWidget.BP_DialogueWidget_C" (Math|Transform|MakeTransform (+ (Transformation|GetActorLocation (Components|GetOwner)) (Variables|Default|GetWidgetOffset)) "0, 0, 0" "1.000000,1.000000,1.000000") "AlwaysSpawn" "MultiplyWithRoot" 0 0))
  (Default|SetupFollowComponent _returnvalue (Components|GetOwner))
  (bind _output_get (Variables|Default|SetDialogueWidget _returnvalue))
  (Class|BPIDialogue|InitialiseDialogue(Message) (Default|GetWidget _output_get) self (Variables|Customise|GetBackground%20Colour%20and%20Opacity) (Variables|Customise|GetText%20Colour%20and%20Opacity)))

(fn GetDialoguePlayTime
  (params (S :type String))
  (return (Math|Float|MapRangeClamped (/ (Math|Conversions|ToFloat(Integer) (Utilities|String|Len S)) (Variables|Autoplay|GetDialogueReadSpeed)) 1.0 1e+01 (Variables|Autoplay|GetMinDialogueTime) (Variables|Autoplay|GetMaxDialogueTime))))