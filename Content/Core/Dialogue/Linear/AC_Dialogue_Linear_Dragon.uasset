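; Linear dialogue component for the dragon NPC, showing speech in a spawned widget actor while a player is detected.
; On detection it spawns the dragon-sized widget at the NPC's WidgetSpawn point; losing detection clears timers and destroys it.
; DT_Dialogue_Dragon rows play in order, broadcasting each line through dispatchers.
; Timers hold lines for a text-based duration with random gaps between them, then advance to the next row.
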(event Custom|DialogueInterval
  ;[1 1 1] Dialogue Interval
  (if (<= (Variables|Default|GetLineIndex) (- (Utilities|Array|Length (Variables|Default|GetOut%20Row%20Dialogue%20Text)) 2))
    (Math|Integer|IncrementInt (Variables|Default|GetLineIndex)
      (:%20%20
        (bind _returnvalue (Utilities|Time|SetTimerbyEvent (EventDispatchers|CreateEvent :!event PlayDialogue) (Math|Random|RandomFloatinRangefromStream (Math|Random|MakeRandomStream (Math|Random|RandomIntegerinRange 0 100)) (Variables|Default|GetMinIntervalDelay) (Variables|Default|GetMaxIntervalDelay))))
        (Variables|Default|SetIntervalHandle _returnvalue)
        (if (not (== (Variables|Default|GetDialogue%20Index) (Utilities|Array|Length (Variables|Default|GetCurrentRowNames))))
          (Default|CallOnDialogueEnded))))
    (else
      ;;[1 1 1] Temp
      (Variables|Default|SetLineIndex 0)
      (Math|Integer|IncrementInt (Variables|Default|GetDialogue%20Index)
        (:%20%20
          (CallFunction|PlayDialogue))))))

(event Custom|StartDialogue
  ;[1 1 1] Start Dialogue
  (CallFunction|EndDialogue)
  (CallFunction|CreateDialogueWidget)
  (CallFunction|PlayDialogue)
  (bind _aswbp_dialogue (Utilities|Casting|CastToWBP_Dialogue (UserInterface|GetUserWidgetObject (Variables|/Game/Core/Dialogue/BP_DialogueWidget.BP_DialogueWidget_C|GetBPW_Dialogue (Variables|Default|GetDialogueWidget)))))
  (Default|UseDragonSize _aswbp_dialogue))

(event Custom|EndDialogue
  ;[1 1 1] End Dialogue
  (Utilities|Time|ClearandInvalidateTimerbyHandle (Variables|Default|GetDialogueHandle))
  (Utilities|Time|ClearandInvalidateTimerbyHandle (Variables|Default|GetConvoHandle))
  (Utilities|IsValid (Variables|Default|GetDialogueWidget)
    (:Is%20Valid
      (Actor|DestroyActor (Variables|Default|GetDialogueWidget))
      (Utilities|Platform|CollectGarbage))))

(event EventBeginPlay
  ;[1 1 1] Begin Play
  (bind _outrownames (DataTable|GetDataTableRowNames "/Game/Core/Dialogue/Linear/DT_Dialogue_Dragon.DT_Dialogue_Dragon"))
  (Variables|Default|SetCurrentRowNames _outrownames))

(event EventOnPlayerDetected
  (params (HasDetected :type Boolean))
  ;[1 1 1] On Player Detected
  (if HasDetected
    (CallFunction|StartDialogue)
    (else
      (CallFunction|EndDialogue))))

(event EventPlayDialogue
  (Development|PrintString "Show Dialogue")
  ;[1 1 1] Play Dialogue
  (bind _returnvalue (Utilities|GetDataTableRow "/Game/Core/Dialogue/Linear/DT_Dialogue_Dragon.DT_Dialogue_Dragon" (Utilities|Array|Get(acopy) (Variables|Default|GetCurrentRowNames) (Variables|Default|GetDialogue%20Index)))
    (:then
      (Variables|Default|SetOut%20Row%20Dialogue%20Text (.dialoguetext _returnvalue))
      (Default|CallOnDialogueUpdated (Utilities|Array|Get(acopy) (Variables|Default|GetOut%20Row%20Dialogue%20Text) (Variables|Default|GetLineIndex)))
      (bind _returnvalue_2 (Utilities|Time|SetTimerbyEvent (delegate Custom|DialogueInterval) (CallFunction|GetDialoguePlayTime (Utilities|String|ToString(Text) (Utilities|Array|Get(acopy) (Variables|Default|GetOut%20Row%20Dialogue%20Text) (Variables|Default|GetLineIndex))))))
      (Variables|Default|SetDialogueHandle _returnvalue_2))))

(fn CreateDialogueWidget
  (bind _asbp_dragon_npc (Utilities|Casting|CastToBP_DragonNPC (Components|GetOwner)))
  (bind _returnvalue (Game|SpawnActorfromClass "/Game/Core/Dialogue/BP_DialogueWidget.BP_DialogueWidget_C" (Math|Transform|MakeTransform (+ (Transformation|GetWorldLocation (Variables|/Game/Art/Textures/Dragon/BP_DragonNPC.BP_DragonNPC_C|GetWidgetSpawn _asbp_dragon_npc)) (Variables|Default|GetWidgetOffset)) "0, 0, 0" "1.000000,1.000000,1.000000") "AlwaysSpawn" "MultiplyWithRoot" 0 0))
  (bind _output_get (Variables|Default|SetDialogueWidget _returnvalue))
  (Class|BPIDialogue|InitialiseDialogue(Message) (Default|GetWidget _output_get) self (Variables|Default|GetBackground%20Colour%20and%20Opacity) (Variables|Default|GetText%20Colour%20and%20Opacity)))