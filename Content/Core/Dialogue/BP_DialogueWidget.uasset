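; BP_DialogueWidget is an actor that displays dialogue through a widget component and trails a target actor.
; On BeginPlay it sets the widget component to a fixed angled relative rotation.
; SetupFollowComponent stores the target, and Tick interpolates the actor toward that target's X and Y while keeping its own height.
; GetWidget returns the component's user widget cast to WBP_Dialogue.
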(event Custom|SetupFollowComponent
  (params (FollowActor :type Actor%20Object%20Reference))
  (Variables|Default|SetFollowActorRef FollowActor))

(event EventTick
  (params (DeltaSeconds :type Float%20%28single-precision%29))
  (bind _followactorref (Variables|Default|GetFollowActorRef))
  (bind _returnvalue (Transformation|GetActorLocation _followactorref))
  (Utilities|IsValid (Variables|Default|GetFollowActorRef)
    (:Is%20Valid
      (Transformation|SetActorLocation (Math|Interpolation|VInterpTo (Transformation|GetActorLocation) (Math|Vector|MakeVector (.x _returnvalue) (.y _returnvalue) (.z (Transformation|GetActorLocation))) (Utilities|Time|GetWorldDeltaSeconds) (Variables|Default|GetInterp%20Speed)) false false))))

(event EventBeginPlay
  (Transformation|SetRelativeRotation (Variables|Default|GetBPW_Dialogue) "45.000000,45.000000,0.000000" false false))

(fn ConstructionScript)

(fn GetWidget
  (return (.AsWBP%20Dialogue (Utilities|Casting|CastToWBP_Dialogue (UserInterface|GetUserWidgetObject (Variables|Default|GetBPW_Dialogue))))))