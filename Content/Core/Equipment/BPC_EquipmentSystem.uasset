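; Equipment system component that manages the player's usable items: invisibility potion, smoke bomb and sleep potion.
; Init stores the player, spawns each configured equipment class as an actor at a fixed location, and initializes it with its matching enabled flag.
; UseItem maps the chosen item to a fixed array index, so it relies on spawn order, and uses that equipment on the player if it allows use.
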(event Custom|Use%20Item
  (params (Using :type E_Equipment%20Enum :default "NewEnumerator0"))
  (bind _returnvalue (Utilities|Select :Index Using :NewEnumerator0 0 :NewEnumerator1 1 :NewEnumerator2 2))
  (bind _equipment (Variables|Default|GetEquipment))
  (bind _output (Utilities|Array|Get(acopy) _equipment _returnvalue))
  (if (Default|CanUseEquipment _output)
    (Default|UseEquipment _output (Variables|Default|GetPlayer))))

(event Custom|Init
  (params (Enabled :type Array%20of%20Booleans) (Player :type BP%20Player%20Character%20Object%20Reference))
  (Variables|Default|SetPlayer Player)
  (for (_array_element _array_index) (Variables|Default|GetEquipmentToSpawn)
    (bind _returnvalue (Game|SpawnActorfromClass _array_element (Math|Transform|MakeTransform "200.000000,200.000000,200.000000") "Undefined" "MultiplyWithRoot" 0 0))
    (Utilities|Array|Add (Variables|Default|GetEquipment) _returnvalue)
    (Default|Init _returnvalue (Utilities|Array|Get(acopy) Enabled _array_index))))