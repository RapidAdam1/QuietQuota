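; Sleep powder equipment that, when used, moves to the player and sprays a particle effect along one of four diagonal directions chosen from their movement direction.
; An enlarged sphere checks overlapping AI characters through CanKillGuard before calling KillBySleep.
; CanKillGuard only prints a facing angle and player distance.
; Its angle-and-distance return is unconnected, so the sleep kill never triggers as wired.
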(event OnComponentBeginOverlap(Sphere)
  (params (OverlappedComponent :type Primitive%20Component%20Object%20Reference) (OtherActor :type Actor%20Object%20Reference) (OtherComp :type Primitive%20Component%20Object%20Reference) (OtherBodyIndex :type Integer) (bFromSweep :type Boolean) (SweepResult :type Hit%20Result%20Structure%20%28by%20ref%29))
  (bind _asai_character (Utilities|Casting|CastToAI_Character OtherActor))
  (bind _cankill (CallFunction|CanKillGuard (Transformation|GetActorTransform _asai_character)))
  (if _cankill
    (Default|KillbySleep _asai_character)))

(event EventUseEquipment
  (params (Interacting%20Player :type BP%20Player%20Character%20Object%20Reference))
  (bind _movementdirection (Variables|/Game/Core/PlayerCharacter/BP_PlayerCharacter.BP_PlayerCharacter_C|GetMovementDirection (Variables|Default|GetInteracting%20Player)))
  (bind _returnvalue (Utilities|Select :Index _movementdirection :NewEnumerator0 "-1.000000,-1.000000,0.000000" :NewEnumerator1 "1.000000,1.000000,0.000000" :NewEnumerator2 "1.000000,-1.000000,0.000000" :NewEnumerator3 "-1.000000,1.000000,0.000000"))
  ;[0 0 0] Item Effect
  (|CallParentFunction Interacting%20Player)
  (if (CallFunction|CanUseEquipment)
    (Transformation|SetActorLocation (Transformation|GetActorLocation (Variables|Default|GetInteracting%20Player)) false false)
    (bind _returnvalue_2 (Niagara|SpawnSystematLocation "/Game/Art/Particle/PS_SleepPowder.PS_SleepPowder" (Transformation|GetWorldLocation (Variables|Default|GetPaperSprite))))
    (Effects|Components|ParticleSystem|SetVectorParameter _returnvalue_2 "FireDirection" _returnvalue)
    (Variables|Default|SetFireDirection _returnvalue)))

(event EventInit
  (params (Enabled :type Boolean))
  (|CallParentFunction Enabled)
  (Components|Sphere|SetSphereRadius (Variables|Default|GetSphere) (* (Variables|Default|GetKillDistance) 2.0) true))

(fn ConstructionScript)

(fn CanKillGuard
  (params (GuardTransform :type Transform))
  (bind _firedirection (Variables|Default|GetFireDirection))
  (bind _rotation (Math|Transform|BreakTransform GuardTransform))
  (bind _location (Math|Transform|BreakTransform GuardTransform))
  (bind _returnvalue (Math|Vector|GetForwardVector _rotation))
  (bind _returnvalue_2 (Math|Vector|GetUnitDirection(Vector) _location _firedirection))
  (bind _returnvalue_3 (Math|Vector|NegateVector _returnvalue))
  (bind (_x _y) (Class|KismetMathLibrary|BreakVector3f _returnvalue_2))
  (bind (_x_2 _y_2) (Class|KismetMathLibrary|BreakVector3f _returnvalue_3))
  (Development|PrintText (Utilities|Text|FormatText "Kill Angle {angle}    Distance: {dist}" (Class|KismetMathLibrary|DegAcos (Math|Vector2D|DotProduct(2D) (Math|Vector2D|MakeVector2D _x _y) (Math|Vector2D|MakeVector2D _x_2 _y_2))) (Math|Vector|Distance(Vector) (.Location (Math|Transform|BreakTransform GuardTransform)) (Transformation|GetActorLocation (Variables|Default|GetInteracting%20Player))))))