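; BP_EquipmentBase is a base equipment actor with use and cooldown handling.
; UseEquipment stores the interacting player, hides the actor, then starts a one-shot cooldown timer if uses remain and it is off cooldown.
; CooldownComplete shows the actor again.
; UseEquipment sets OnCooldown false rather than true, so that flag blocks nothing here, and Uses is never decremented in this graph.
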(event Custom|CooldownComplete
  (Variables|Default|SetOnCooldown false)
  (Rendering|SetActorHiddenInGame false)
  (Development|PrintString (Utilities|String|Append (Utilities|GetDisplayName self) "   " "CooldownEnded") false false))

(event Custom|Init
  (params (Enabled :type Boolean))
  (Variables|Default|SetEnabled Enabled))

(event EventUseEquipment
  (params (Interacting%20Player :type BP%20Player%20Character%20Object%20Reference))
  (Variables|Default|SetInteracting%20Player Interacting%20Player)
  (Rendering|SetActorHiddenInGame true)
  (if (CallFunction|CanUseEquipment)
    (bind _returnvalue (Utilities|Time|SetTimerbyEvent (EventDispatchers|CreateEvent :!event Custom|CooldownComplete) (Variables|Default|GetCooldownTime)))
    (Variables|Default|SetCooldown_Timer _returnvalue)
    (Variables|Default|SetOnCooldown false)
    (Development|PrintString (Utilities|String|Append (Utilities|GetDisplayName self) "   " "CooldownStarte") false false)))

(fn ConstructionScript)

(fn CanUseEquipment
  (return (and (!= (Variables|Default|GetUses) 0) (not (Variables|Default|GetOnCooldown)))))