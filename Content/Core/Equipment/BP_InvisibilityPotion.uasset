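; Invisibility potion equipment that, when usable, makes the interacting player undetectable and nearly transparent for the item effect duration.
; Use disables CanBeDetected on the player's detection component, starts a timer and applies a dynamic translucent material instance to the Paper flipbook at low opacity.
; Deactivation restores detectability and full opacity, clears the timer and destroys the potion actor.
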(event Custom|SetInvisMaterial
  (params (SetEnabled :type Boolean))
  ;[1 1 1] Set Invis Material
  (if SetEnabled
    (bind _returnvalue (Rendering|Material|CreateDynamicMaterialInstance (Variables|/Game/Core/PlayerCharacter/BP_PlayerCharacter.BP_PlayerCharacter_C|GetPaperFlipbook (Variables|Default|GetInteracting%20Player)) 0 "/Game/Art/Materials/M_TranslucentSprite.M_TranslucentSprite" "None" :!class /Script/Engine.PrimitiveComponent))
    (bind _output_get (Variables|Default|SetPlayerMaterial _returnvalue))
    (Rendering|Material|SetScalarParameterValue _output_get "NewOpacity" 0.1 :!class /Script/Engine.MaterialInstanceDynamic)
    (else
      (Rendering|Material|SetScalarParameterValue (Variables|Default|GetPlayerMaterial) "NewOpacity" 1.0 :!class /Script/Engine.MaterialInstanceDynamic))))

(event Custom|Potion%20Duration
  (params (potion%20activated? :type Boolean) (Duration :type Float%20%28double-precision%29))
  ;[0 0 0] Potion Duration
  (if potion%20activated?
    (bind _returnvalue (Utilities|Time|SetTimerbyEvent (EventDispatchers|CreateEvent :!event Custom|Deactivate%20Potion) Duration))
    (Variables|Default|SetPotion%20Timer%20Handle _returnvalue)
    (CallFunction|SetInvisMaterial true)))

(event Custom|Deactivate%20Potion
  ;[0 0 0] Deactivate Potion
  (Variables|/Game/Core/AI/AI_AwarenessSystem/AC_PlayerDetectionComponent.AC_PlayerDetectionComponent_C|SetCanBeDetected (Variables|/Game/Core/PlayerCharacter/BP_PlayerCharacter.BP_PlayerCharacter_C|GetAC_PlayerDetectionComponent (Variables|Default|GetInteracting%20Player)) true)
  (CallFunction|SetInvisMaterial false)
  (Utilities|Time|ClearandInvalidateTimerbyHandle (Variables|Default|GetPotion%20Timer%20Handle))
  (Development|PrintString "Potion Deactivated" false false "(R=1.000000,G=0.000000,B=0.051567,A=1.000000)")
  (Actor|DestroyActor))

(event EventBeginPlay
  (|CallParentFunction) ; This node is disabled and will not be called.\nDrag off pins to build functionality.
)

(event Collision|EventActorBeginOverlap
  (params (OtherActor :type Actor%20Object%20Reference))
  (|CallParentFunction OtherActor) ; This node is disabled and will not be called.\nDrag off pins to build functionality.
)

(event EventTick
  (params (DeltaSeconds :type Float%20%28single-precision%29))
  (|CallParentFunction DeltaSeconds) ; This node is disabled and will not be called.\nDrag off pins to build functionality.
)

(event EventUseEquipment
  (params (Interacting%20Player :type BP%20Player%20Character%20Object%20Reference))
  ;[0 0 0] Item Effect
  (|CallParentFunction Interacting%20Player)
  (if (CallFunction|CanUseEquipment)
    (Variables|/Game/Core/AI/AI_AwarenessSystem/AC_PlayerDetectionComponent.AC_PlayerDetectionComponent_C|SetCanBeDetected (Variables|/Game/Core/PlayerCharacter/BP_PlayerCharacter.BP_PlayerCharacter_C|GetAC_PlayerDetectionComponent Interacting%20Player) false)
    (Development|PrintString (Utilities|String|ToString(Float) (Variables|Default|GetItemEffectDuration)) false false "(R=0.000000,G=1.000000,B=0.185984,A=1.000000)" 1e+01)
    (CallFunction|PotionDuration true (Variables|Default|GetItemEffectDuration))))

(fn ConstructionScript
  (|CallParentFunction))