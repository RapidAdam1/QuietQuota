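; BP_SmokeBomb is an equipment item that hides the player who uses it from detection inside a smoke cloud.
; On use it moves to that player, spawns the smoke effect and starts a duration timer.
; Overlapping its radius-sized sphere disables that player's detection and zeroes awareness through their detection component, and leaving restores detectability.
; An end-timer event also restores detectability, then destroys the actor.
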(event OnComponentBeginOverlap(Sphere)
  (params (OverlappedComponent :type Primitive%20Component%20Object%20Reference) (OtherActor :type Actor%20Object%20Reference) (OtherComp :type Primitive%20Component%20Object%20Reference) (OtherBodyIndex :type Integer) (bFromSweep :type Boolean) (SweepResult :type Hit%20Result%20Structure%20%28by%20ref%29))
  (if (== OtherActor (Variables|Default|GetInteracting%20Player))
    (CallFunction|EnterSmoke)))

(event OnComponentEndOverlap(Sphere)
  (params (OverlappedComponent :type Primitive%20Component%20Object%20Reference) (OtherActor :type Actor%20Object%20Reference) (OtherComp :type Primitive%20Component%20Object%20Reference) (OtherBodyIndex :type Integer))
  (if (== OtherActor (Variables|Default|GetInteracting%20Player))
    (CallFunction|ExitSmoke)))

(event Custom|SmokeBombEndTimer
  (CallFunction|ExitSmoke)
  (Actor|DestroyActor))

(event Custom|Enter%20Smoke
  (bind _interacting_player (Variables|Default|GetInteracting%20Player))
  (bind _ac_playerdetectioncomponent (Variables|/Game/Core/PlayerCharacter/BP_PlayerCharacter.BP_PlayerCharacter_C|GetAC_PlayerDetectionComponent _interacting_player))
  (Variables|/Game/Core/AI/AI_AwarenessSystem/AC_PlayerDetectionComponent.AC_PlayerDetectionComponent_C|SetCanBeDetected _ac_playerdetectioncomponent false)
  (Variables|/Game/Core/AI/AI_AwarenessSystem/AC_PlayerDetectionComponent.AC_PlayerDetectionComponent_C|SetCurrentAwareness _ac_playerdetectioncomponent 0.0))

(event Custom|ExitSmoke
  (Variables|/Game/Core/AI/AI_AwarenessSystem/AC_PlayerDetectionComponent.AC_PlayerDetectionComponent_C|SetCanBeDetected (Variables|/Game/Core/PlayerCharacter/BP_PlayerCharacter.BP_PlayerCharacter_C|GetAC_PlayerDetectionComponent (Variables|Default|GetInteracting%20Player)) true))

(event EventUseEquipment
  (params (Interacting%20Player :type BP%20Player%20Character%20Object%20Reference))
  ;[0 0 0] Item Effect
  (|CallParentFunction Interacting%20Player)
  (if (CallFunction|CanUseEquipment)
    (Transformation|SetActorLocation (Transformation|GetActorLocation (Variables|Default|GetInteracting%20Player)) false false)
    (bind _returnvalue (Utilities|Time|SetTimerbyEvent (EventDispatchers|CreateEvent :!event Custom|SmokeBombEndTimer) 0.0 false (Variables|Default|GetDuration)))
    (Variables|Default|SetTimer _returnvalue)
    (Niagara|SpawnSystematLocation "/Game/Art/Particle/PS_SmokeCloud.PS_SmokeCloud" (Transformation|GetWorldLocation (Variables|Default|GetPaperSprite)))))

(event EventInit
  (params (Enabled :type Boolean))
  (|CallParentFunction Enabled)
  (Components|Sphere|SetSphereRadius (Variables|Default|GetSphere) (Variables|Default|GetRadius) true))

(fn ConstructionScript)