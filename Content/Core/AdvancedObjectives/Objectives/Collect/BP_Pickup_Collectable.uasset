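; Collectable pickup for the Collect objective, shown as a Paper2D sprite that is set through InitSprite.
; TestPickup fires the OnPickup call, plays a 2D sound, spawns an emitter and then destroys the actor.
; AddMinimapIcon creates a scaled AC_Minimap_Collect component and stores it as the pickup's MinimapIcon.
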(event Custom|TestPickup
  (Default|CallOnPickup)
  ;[1 1 1] Effects
  (Audio|PlaySound2D 0 1.0 1.0 0.0 0 0)
  (Effects|SpawnEmitteratLocation 0 "0, 0, 0")
  (Actor|DestroyActor))

(event Custom|Init%20Sprite
  (params (Sprite :type Paper%20Sprite%20Object%20Reference))
  (Rendering|Components|Sprite|SetSprite (Variables|Default|GetPaperSprite) Sprite))

(fn ConstructionScript
  (|CallParentFunction))

(fn AddMinimapIcon
  (bind _returnvalue (Game|AddComponentbyClass "/Game/Core/Minimap/AC_Minimap_Collect.AC_Minimap_Collect_C" false (Math|Transform|MakeTransform "0, 0, 0" "0, 0, 0" "4.000000,4.000000,1.000000")))
  (Variables|Default|SetMinimapIcon _returnvalue))