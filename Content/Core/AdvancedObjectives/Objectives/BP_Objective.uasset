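; BP_Objective is an objective in the AdvancedObjectives system that tracks whether it is required and whether it is completed.
; Init stores the required flag, and CompleteObjective marks completion once, then calls OnCompleted with itself.
; GetUIData returns the Sequences for UI.
; NextSequence is an empty event, and a last-index check leading to CompleteObjective is left unconnected, so sequences do not advance here.
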(event Custom|Complete%20Objective
  (if (not (Variables|Default|GetCompleted))
    (Variables|Default|SetCompleted true)
    (Default|CallOnCompleted self)))

(event Custom|Init
  (params (Required%20Objective :type Boolean))
  (Variables|Default|SetRequired Required%20Objective))

(event Custom|NextSequence
  (params (Sequence :type Integer)))

(fn ConstructionScript)

(fn GetUIData
  (return (Variables|Default|GetSequences)))