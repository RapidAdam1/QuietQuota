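; BP_ObjectiveEnd is an end-of-level objective that finishes the level when the player enters its collision volume.
; A one-shot overlap casts to BP_PlayerCharacter, updates its animation, disables input, removes the minimap icon and signals objective completion.
; After a short delay it saves through the game instance cached at BeginPlay and loads another level.
; AddMinimapIcon attaches an enlarged level-end minimap component as the objective's icon.
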(event OnComponentBeginOverlap(Collision_Overlap)
  (params (OverlappedComponent :type Primitive%20Component%20Object%20Reference) (OtherActor :type Actor%20Object%20Reference) (OtherComp :type Primitive%20Component%20Object%20Reference) (OtherBodyIndex :type Integer) (bFromSweep :type Boolean) (SweepResult :type Hit%20Result%20Structure%20%28by%20ref%29))
  (bind _gameinstanceref (Variables|Default|GetGameInstanceRef))
  (Utilities|FlowControl|DoOnce false
    (:Completed
      (bind _asbp_player_character (Utilities|Casting|CastToBP_PlayerCharacter OtherActor))
      (Default|UpdateAnimation _asbp_player_character true)
      (Input|DisableInput _asbp_player_character (Game|GetPlayerController 0))
      (CallFunction|RemoveMinimapIcon)
      (Default|CallOnComplete)
      (Utilities|FlowControl|Delay 2.0)
      (Default|SaveData _gameinstanceref true)
      (Default|LoadLevel _gameinstanceref "NewEnumerator0"))))

(event EventBeginPlay
  (bind _asgi_quiet_quota_instance (Utilities|Casting|CastToGI_QuietQuota_Instance (Game|GetGameInstance)))
  (Variables|Default|SetGameInstanceRef _asgi_quiet_quota_instance))

(fn ConstructionScript)

(fn AddMinimapIcon
  (bind _returnvalue (Game|AddComponentbyClass "/Game/Core/Minimap/AC_Minimap_LevelEnd.AC_Minimap_LevelEnd_C" false (Math|Transform|MakeTransform "0, 0, 0" "0, 0, 0" "4.000000,4.000000,4.000000")))
  (Variables|Default|SetMinimapIcon _returnvalue))