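; BP_ObjectiveManager spawns and tracks a level's objectives, then opens the escape phase once enough required ones are completed.
; BeginPlay records the player's start transform and creates an informant objective, while StartObjectives adds random required objectives from the level list.
; Completion events count toward the target, then spawn an end objective at that saved transform and save the game.
; Main and optional objective creation is disconnected.
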(event Custom|Escape%20Level%20Sequence
  (bind _levelendtransform (Variables|Default|GetLevelEndTransform))
  ;[1 1 1] Escape Level Sequence
  (Utilities|Array|Clear (Variables|Default|GetObjectives))
  (bind _returnvalue (Game|SpawnActorfromClass "/Game/Core/AdvancedObjectives/BP_ObjectiveEnd.BP_ObjectiveEnd_C" (Math|Transform|MakeTransform (.location _levelendtransform) (.rotation _levelendtransform) "2.000000,2.000000,2.000000") "AdjustIfPossibleButAlwaysSpawn" "MultiplyWithRoot" 0 0))
  (Default|CallOnObjectivesComplete _returnvalue)
  (Class|BPIObjectiveTarget|SetasObjectiveTarget(Message) _returnvalue true)
  (Default|SaveGame (Variables|Default|GetSaveSystem)))

(event Custom|OnObjectiveCompleted
  (params (Objective :type BP%20Objective%20Object%20Reference))
  ;[1 1 1] Objective Completion
  (if (Variables|/Game/Core/AdvancedObjectives/Objectives/BP_Objective.BP_Objective_C|GetRequired Objective)
    ;;[1 1 1] Required
    (Math|Integer|IncrementInt (Variables|Default|GetObjectives%20Completed)
      (:%20%20
        (if (>= (Variables|Default|GetObjectives%20Completed) (Variables|Default|GetObjectives%20Required))
          (CallFunction|EscapeLevelSequence)
          (else
            (CallFunction|UpdateObjectiveUI)))))
    (else
      ;;[1 1 1] Optional
      (Development|PrintString "Optional Objective Completed" false false))))

(event Custom|Update%20Objective%20UI)

(event Custom|Initialise
  (params (Main%20Objective :type BP%20Objective%20Class%20Reference) (Required%20Objectives :type Integer) (Optional%20Objectives :type Integer))
  (Utilities|FlowControl|Sequence
    (:then_0
      ;[1 1 1] Create Required Objectives
      (for _index (range 0 (- Required%20Objectives 1))
        (bind _class (CallFunction|GetObjectiveClass true))
        (CallFunction|CreateObjective _class true)))))

(event Custom|Create%20Objective
  (params (Objective%20Class :type BP%20Objective%20Class%20Reference) (Required :type Boolean))
  ;[1 1 1] Create Objective & Init
  (bind _returnvalue (Game|SpawnActorfromClass Objective%20Class (Transformation|GetActorTransform) "Undefined" "MultiplyWithRoot" 0 0))
  (Utilities|Array|Add (Variables|Default|GetObjectives) _returnvalue)
  (Default|Init _returnvalue Required)
  (EventDispatchers|BindEventtoOnCompleted _returnvalue (EventDispatchers|CreateEvent :!event Custom|OnObjectiveCompleted))
  (Default|CallOnObjectiveAssigned (select Required (Variables|Default|GetCurrentRequired) (Variables|Default|GetCurrentOptional)) Required))

(event Custom|StartObjectives
  ;[1 1 1] Start Objectives
  (CallFunction|Initialise "/Game/Core/AdvancedObjectives/Objectives/Assassinate/Objective_Assassinate.Objective_Assassinate_C" (Variables|Default|GetObjectives%20Required) (Variables|Default|GetOptional%20Objectives)))

(event EventBeginPlay
  ;[1 1 1] Begin Play
  (Variables|Default|SetLevelEndTransform (Transformation|GetActorTransform (Game|Player|GetPlayerPawn 0)))
  (CallFunction|CreateObjective "/Game/Core/AdvancedObjectives/Objectives/Informant/Objective_Informant.Objective_Informant_C" true)
  (bind _returnvalue (Game|SpawnActorfromClass "/Game/Core/SafeRoom/SaveAccessorTest.SaveAccessorTest_C" (Math|Transform|MakeTransform "0, 0, 0" "0, 0, 0" "1.000000,1.000000,1.000000") "AlwaysSpawn" "MultiplyWithRoot" 0 0))
  (Variables|Default|SetSaveSystem _returnvalue))

(fn ConstructionScript)

(fn GetObjectiveClass
  (params (Is%20Required :type Boolean))
  (if Is%20Required
    (bind _output_get (Variables|Default|SetCurrentRequired (.OutItem (Utilities|Array|Random (Variables|/Game/Core/AdvancedObjectives/DA_Objectives.DA_Objectives_C|GetRequired (Variables|Default|GetLevel_ObjectiveList))))))
    (LocalVariables|SetDesiredClass (.Class (Utilities|Struct|BreakObjective_Data _output_get)))
    (else
      (bind _output_get_2 (Variables|Default|SetCurrentOptional (.OutItem (Utilities|Array|Random (Variables|/Game/Core/AdvancedObjectives/DA_Objectives.DA_Objectives_C|GetOptional (Variables|Default|GetLevel_ObjectiveList))))))
      (LocalVariables|SetDesiredClass (.Class (Utilities|Struct|BreakObjective_Data _output_get_2)))))
  (if (Utilities|IsValidClass (LocalVariables|GetDesiredClass))
    (return (LocalVariables|GetDesiredClass))
    (else
      (Development|PrintString "Failed To Find Valid Objective Class" false false)
      (return "/Game/Core/AdvancedObjectives/Objectives/BP_Objective.BP_Objective_C"))))